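; Blueprint interface that interactive objects implement to respond to player interaction.
; It declares main and secondary actions, each with press, hold with elapsed time, and hold-reset functions; the main press receives a hit result and its hold a direction.
; Hover and focus start and end events complete the contract, alongside boolean queries reporting whether interaction, each action or hold, and focus are available.
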(fn DoMainAction
  (params (HitResult :type Hit%20Result%20Structure)))

(fn DoMainActionHold
  (params (HoldTime :type Float%20%28double-precision%29) (Direction :type Vector%202D%20Structure)))

(fn DoMainActionHoldReset)

(fn DoSecondAction)

(fn DoSecondActionHold
  (params (HoldTime :type Float%20%28double-precision%29)))

(fn DoSecondActionHoldReset)

(fn OnHoverStart)

(fn OnHoverEnd)

(fn IsInteractionAvailable
  (return false))

(fn IsMainActionAvailable
  (return false))

(fn IsMainHoldActionAvailable
  (return false))

(fn IsSecondActionAvailable
  (return false))

(fn IsSecondHoldActionAvailable
  (return false))

(fn OnFocusStart)

(fn OnFocusEnd)

(fn IsFocusAvailable
  (return false))
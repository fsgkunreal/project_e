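; BP_TestInteractive is a test actor for an interaction interface that highlights its Cube mesh while hovered.
; OnHoverStart applies the M_Overlay overlay material and OnHoverEnd clears it, each printing a debug string.
; Its availability functions report focus and interaction as available, while all main and secondary press and hold actions are unavailable.
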(event EventBeginPlay)

(event Collision|EventActorBeginOverlap
  (params (OtherActor :type Actor%20Object%20Reference)))

(event EventTick
  (params (DeltaSeconds :type Float%20%28single-precision%29)))

(event EventOnHoverEnd
  (Development|PrintString "HoverEnd")
  (Rendering|Material|SetOverlayMaterial (Variables|Default|GetCube) 0 :!class /Script/Engine.MeshComponent))

(event EventOnHoverStart
  (Development|PrintString "HoverStart")
  (Rendering|Material|SetOverlayMaterial (Variables|Default|GetCube) "/Game/content_0/interfaces/M_Overlay.M_Overlay" :!class /Script/Engine.MeshComponent))

(fn ConstructionScript)

(fn IsFocusAvailable
  (return true))

(fn IsInteractionAvailable
  (return true))

(fn IsMainActionAvailable
  (return false))

(fn IsMainHoldActionAvailable
  (return false))

(fn IsSecondActionAvailable
  (return false))

(fn IsSecondHoldActionAvailable
  (return false))
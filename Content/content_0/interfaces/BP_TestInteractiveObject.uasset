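; BP_TestInteractiveObject is a test interactive object that reports each interaction it receives through on-screen debug prints.
; Main and second action events, each with tap, hold and hold-reset variants, print their names.
; Hover start applies M_Overlay as the static mesh overlay material to highlight it, and hover end clears it, both logging under a shared print key.
; Two leftover highlight on/off prints are disconnected.
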(event EventOnHoverStart
  (Rendering|Material|SetOverlayMaterial (Variables|Default|GetStaticMesh) "/Game/content_0/interfaces/M_Overlay.M_Overlay" :!class /Script/Engine.MeshComponent)
  (Development|PrintString "OnHoverStart" true true "(R=1.000000,G=0.968910,B=0.000000,A=1.000000)" 2.0 "3"))

(event EventOnHoverEnd
  (Rendering|Material|SetOverlayMaterial (Variables|Default|GetStaticMesh) 0 :!class /Script/Engine.MeshComponent)
  (Development|PrintString "OnHoverEnd" true true "(R=1.000000,G=0.968910,B=0.000000,A=1.000000)" 2.0 "3"))

(event EventDoMainActionHoldReset
  (Development|PrintString "Main Action (Hold Reset)"))

(event EventDoSecondAction
  (Development|PrintString "Second Action (Tap)" true true "(R=1.000000,G=0.019054,B=0.000000,A=1.000000)"))

(event EventDoSecondActionHold
  (params (HoldTime :type Float%20%28double-precision%29))
  (Development|PrintString "Second Action (Hold)" true true "(R=1.000000,G=0.019054,B=0.000000,A=1.000000)"))

(event EventDoSecondActionHoldReset
  (Development|PrintString "Second Action (Hold Reset)" true true "(R=1.000000,G=0.019054,B=0.000000,A=1.000000)"))

(event EventDoMainAction
  (Development|PrintString "Main Action (Tap)"))

(event EventDoMainActionHold
  (params (HoldTime :type Float%20%28double-precision%29))
  (Development|PrintString "Main Action (Hold)"))

(fn ConstructionScript)
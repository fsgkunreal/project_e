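; Focusable cabinet that gathers its child BP_Drawer actors and spawns an item from a random one at BeginPlay.
; Hovering toggles an outline overlay and Niagara effect on the cabinet and drawers; focusing turns on a light and enables drawer interaction.
; On gamepad only, additional-action input steps through drawer indices, Tick moves the highlight to match, and the second action operates the selected drawer.
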(event EventDoAdditionalAction
  (params (Input :type Float%20%28double-precision%29))
  ;[0.3177 0.3177 0.3177 0.313] MainAction
  (bind _bisgamepad (CallFunction|GetControllerLayout))
  (if _bisgamepad
    (CallFunction|ChangeDraweronHover Input)))

(event EventDoSecondAction
  (params (HitResult :type Hit%20Result%20Structure))
  ;[0.3177 0.3177 0.3177 0.313] MainAction
  (if (Variables|Default|GetbIsOnFocus)
    (bind _bisgamepad (CallFunction|GetControllerLayout))
    (if _bisgamepad
      (Default|DrawerInteraction (Variables|Default|GetDrawerOnHover)))))

(event EventTick
  (params (DeltaSeconds :type Float%20%28single-precision%29))
  (bind _drawerarray (Variables|Default|GetDrawerArray))
  (bind _drawerindex (Variables|Default|GetDrawerIndex))
  (bind _output (Utilities|Array|Get(acopy) _drawerarray _drawerindex))
  ;[0.3177 0.3177 0.3177 0.313] EvenTick
  (if (Variables|Default|GetbIsOnFocus)
    (bind _bisgamepad (CallFunction|GetControllerLayout))
    (if _bisgamepad
      (if (!= (Variables|Default|GetDrawerOnHover) _output)
        (Default|ApplyonHoverEffect (Variables|Default|GetDrawerOnHover) false)
        (bind _output_get (Variables|Default|SetDrawerOnHover _output))
        (Default|ApplyonHoverEffect _output_get true)))))

(event EventBeginPlay
  (bind _drawerarray (Variables|Default|GetDrawerArray))
  ;[0.3177 0.3177 0.3177 0.313] BeginPlay
  (for _array_element (Actor|GetAllChildActors true)
    (bind _asbp_drawer (Utilities|Casting|CastToBP_Drawer _array_element))
    (Utilities|Array|Add (Variables|Default|GetDrawerArray) _asbp_drawer))
  (Variables|Default|SetDrawerOnHover (Utilities|Array|Get(acopy) _drawerarray (Variables|Default|GetDrawerIndex)))
  (bind _item (Default|SpawnItem (.OutItem (Utilities|Array|Random _drawerarray))))
  (Variables|Default|SetItemInDrawer _item))

(event EventOnHoverStart
  ;[0.3177 0.3177 0.3177 0.313] HoverAndFocus
  (if (Variables|Default|GetbIsOnFocus)
    (CallFunction|ApplyonHoverEffect false)
    (else
      (CallFunction|ApplyonHoverEffect true))))

(event EventOnHoverEnd
  ;[0.3177 0.3177 0.3177 0.313] HoverAndFocus
  (CallFunction|ApplyonHoverEffect false))

(event EventOnFocusStart
  ;[0.3177 0.3177 0.3177 0.313] HoverAndFocus
  (bind _output_get (Variables|Default|SetbIsOnFocus true))
  (Rendering|SetVisibility (Variables|Default|GetLight) _output_get false)
  (Utilities|FlowControl|Sequence
    (:then_0
      (CallFunction|ApplyonHoverEffect false))
    (:then_1
      (CallFunction|DrawerInteractionHandler _output_get)
      (bind _bisgamepad (CallFunction|GetControllerLayout))
      (if _bisgamepad
        (Default|ApplyonHoverEffect (Variables|Default|GetDrawerOnHover) true)))))

(event EventOnFocusEnd
  ;[0.3177 0.3177 0.3177 0.313] HoverAndFocus
  (bind _output_get (Variables|Default|SetbIsOnFocus false))
  (Rendering|SetVisibility (Variables|Default|GetLight) _output_get false)
  (CallFunction|DrawerInteractionHandler _output_get)
  (Default|ApplyonHoverEffect (Variables|Default|GetDrawerOnHover) false)
  (bind _bisgamepad (CallFunction|GetControllerLayout))
  (CallFunction|ApplyonHoverEffect _bisgamepad))

(fn ConstructionScript
  (bind _staticmesh (Variables|Default|GetStaticMesh))
  (Utilities|IsValid _staticmesh
    (:Is%20Valid
      (Components|StaticMesh|SetStaticMesh (Variables|Default|GetBody) _staticmesh))))

(fn ApplyonHoverEffect
  (params (bIsOnHoverStart :type Boolean))
  (bind _drawerarray (Variables|Default|GetDrawerArray))
  (if bIsOnHoverStart
    (Rendering|Material|SetOverlayMaterial (Variables|Default|GetBody) "/Game/content_2/InteractiveObject/Effects/MI_Outline.MI_Outline" :!class /Script/Engine.MeshComponent)
    (Components|Activation|SetActive (Variables|Default|GetNiagara) true false)
    (for _array_element _drawerarray
      (Default|ApplyonHoverEffect _array_element true))
    (else
      (Rendering|Material|SetOverlayMaterial (Variables|Default|GetBody) 0 :!class /Script/Engine.MeshComponent)
      (Components|Activation|Deactivate (Variables|Default|GetNiagara))
      (for _array_element_2 _drawerarray
        (Default|ApplyonHoverEffect _array_element_2 false)))))

(fn DrawerInteractionHandler
  (params (bIsInteractionAvailable :type Boolean))
  (for _array_element (Variables|Default|GetDrawerArray)
    (Default|InteractionHandler _array_element bIsInteractionAvailable)))

(fn GetControllerLayout
  (bind _asmy_game_instance (Utilities|Casting|CastToMyGameInstance (Game|GetGameInstance)))
  (switch Utilities|FlowControl|Switch|SwitchonE_ControlLayout (Default|GetControlLayout _asmy_game_instance)
    (:NewEnumerator0
      _)
    (:NewEnumerator1
      _)
    (:NewEnumerator2
      (return true)))
  (return false))

(fn ChangeDraweronHover
  (params (Input :type Float%20%28double-precision%29))
  (if (< Input 0.0)
    (if (<= (+ (Variables|Default|GetDrawerIndex) 1) (- (Utilities|Array|Length (Variables|Default|GetDrawerArray)) 1))
      (Variables|Default|SetDrawerIndex (+ (Variables|Default|GetDrawerIndex) 1)))
    (elif (>= (- (Variables|Default|GetDrawerIndex) 1) 0)
      (Variables|Default|SetDrawerIndex (- (Variables|Default|GetDrawerIndex) 1)))))

(fn IsFocusAvailable
  (return true))

(fn IsInteractionAvailable
  (return true))

(fn IsMainActionAvailable
  (return true))

(fn IsMainHoldActionAvailable
  (return false))

(fn IsSecondActionAvailable
  (return true))

(fn IsSecondHoldActionAvailable
  (return false))
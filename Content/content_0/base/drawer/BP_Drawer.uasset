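; Interactable drawer that outlines on hover and slides open or closed on main or second action, with sound.
; DrawerInteraction picks the target from which half of the travel it sits in; Tick eases local Y there with FInterpTo until AnimationDrawerHandler stops it.
; Construction applies an optional mesh override.
; Gamepad slide, screen-space open direction and bottle spawn helpers are uncalled here; mouse drag is an empty stub with disconnected grab logic.
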(event EventBeginPlay)

(event EventDoSecondAction
  (params (HitResult :type Hit%20Result%20Structure))
  (CallFunction|DrawerInteraction))

(event EventDoMainAction
  (params (HitResult :type Hit%20Result%20Structure))
  (CallFunction|DrawerInteraction))

(event EventTick
  (params (DeltaSeconds :type Float%20%28single-precision%29))
  (CallFunction|UpdateDrawerRelativeLocation (Variables|Default|GetbIsDrawerAnimation)))

(event EventOnHoverStart
  (params (CurrentControlLayout :type E_ControlLayout%20Enum :default "NewEnumerator0"))
  (if (Variables|Default|GetbIsInteractionAvailable)
    (Rendering|Material|SetOverlayMaterial (Variables|Default|GetDrawer) "/Game/content_2/InteractiveObject/Effects/MI_Outline.MI_Outline" :!class /Script/Engine.MeshComponent)))

(event EventOnHoverEnd
  (params (CurrentControlLayout :type E_ControlLayout%20Enum :default "NewEnumerator0"))
  (if (Variables|Default|GetbIsInteractionAvailable)
    (Rendering|Material|SetOverlayMaterial (Variables|Default|GetDrawer) 0 :!class /Script/Engine.MeshComponent)))

(event EventDoMainActionHold
  (params (HoldTime :type Float%20%28double-precision%29) (Direction :type Vector%202D%20Structure)))

(event EventDoMainActionHoldReset)

(fn ConstructionScript
  (bind _staticmesh (Variables|Default|GetStaticMesh))
  (Utilities|IsValid _staticmesh
    (:Is%20Valid
      (Components|StaticMesh|SetStaticMesh (Variables|Default|GetDrawer) _staticmesh))))

(fn SpawnItem
  (bind _returnvalue (Game|SpawnActorfromClass "/Game/content_2/ThrowableObject/BP_Throwable_Samll_Bottle_1.BP_Throwable_Samll_Bottle_1_C" (Math|Conversions|ToTransform(Vector) (.Origin (Collision|GetComponentBounds (Variables|Default|GetDrawer)))) "AdjustIfPossibleButAlwaysSpawn" "MultiplyWithRoot" 0 0))
  (Physics|SetSimulatePhysics (Variables|/Game/content_0/base/throwable/BP_Throwable.BP_Throwable_C|GetMesh _returnvalue) false)
  (return _returnvalue))

(fn GamepadDrawerInteraction
  (params (Slide :type Float%20%28double-precision%29))
  (bind _drawer (Variables|Default|GetDrawer))
  (Transformation|SetRelativeLocation _drawer (Math|Vector|MakeVector 0.0 (Math|Float|Clamp(Float) (+ Slide (.y (Variables|/Script/Engine.SceneComponent|GetRelativeLocation _drawer))) (Variables|Default|GetMinSlideDistance) (Variables|Default|GetMaxSlideDistance)) 0.0) false false))

(fn InteractionHandler
  (params (bIsInteractionAvailable :type Boolean))
  (Variables|Default|SetbIsInteractionAvailable bIsInteractionAvailable))

(fn MouseDrawerInteraction)

(fn GetOpenDirection
  (bind _returnvalue (Game|GetPlayerController 0))
  (bind _drawer (Variables|Default|GetDrawer))
  (bind _returnvalue_2 (Transformation|GetWorldLocation _drawer))
  (return (Math|Vector2D|Normalize2D (- (.ScreenPosition (Class|GameplayStatics|ProjectWorldtoScreen _returnvalue (+ _returnvalue_2 (* (Transformation|GetActorForwardVector) 1e+02)) false)) (.ScreenPosition (Class|GameplayStatics|ProjectWorldtoScreen _returnvalue _returnvalue_2 false))))))

(fn ApplyonHoverEffect
  (params (bIsHoverStart :type Boolean))
  (if bIsHoverStart
    (Rendering|Material|SetOverlayMaterial (Variables|Default|GetDrawer) "/Game/content_2/InteractiveObject/Effects/MI_Outline.MI_Outline" :!class /Script/Engine.MeshComponent)
    (else
      (Rendering|Material|SetOverlayMaterial (Variables|Default|GetDrawer) 0 :!class /Script/Engine.MeshComponent))))

(fn UpdateDrawerRelativeLocation
  (params (bIsDrawerAnimation :type Boolean))
  (if bIsDrawerAnimation
    (bind _output_get (Variables|Default|SetSlideLocation (Math|Interpolation|FInterpTo (.y (Variables|/Script/Engine.SceneComponent|GetRelativeLocation (Variables|Default|GetDrawer))) (Variables|Default|GetTempSlideLocation) (Utilities|Time|GetWorldDeltaSeconds) 6.0)))
    (Transformation|SetRelativeLocation (Variables|Default|GetDrawer) (Math|Vector|MakeVector 0.0 _output_get 0.0) false false)
    (Utilities|AnimationDrawerHandler false false)))

(fn DrawerInteraction
  (if (Math|Float|InRange(Float) (.y (Variables|/Script/Engine.SceneComponent|GetRelativeLocation (Variables|Default|GetDrawer))) 0.0 (/ (Variables|Default|GetMaxSlideDistance) 2.0))
    (Variables|Default|SetTempSlideLocation (Variables|Default|GetMaxSlideDistance))
    (Audio|Components|Audio|Play (Variables|Default|GetOpenDrawer) 0.0)
    (else
      (Variables|Default|SetTempSlideLocation (Variables|Default|GetMinSlideDistance))
      (Audio|Components|Audio|Play (Variables|Default|GetCloseDrawer) 0.0)))
  (Utilities|AnimationDrawerHandler true false))

(fn IsFocusAvailable
  (return false))

(fn IsInteractionAvailable
  (return (Variables|Default|GetbIsInteractionAvailable)))

(fn IsMainActionAvailable
  (return true))

(fn IsMainHoldActionAvailable
  (return true))

(fn IsSecondActionAvailable
  (return true))

(fn IsSecondHoldActionAvailable
  (return false))
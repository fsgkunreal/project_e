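; Player camera pawn that moves along its own forward and right axes, rotates in yaw and zooms through a spring arm.
; Scroll input sets a clamped target zoom, which Tick eases toward, scaling move speed and gamepad trace radius from the current arm length.
; Focus events blend the view to a target actor and back to the player pawn, while card use only prints the slot name.
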(event Custom|ScrollCam
  (params (Step :type Float%20%28double-precision%29))
  ;[0.1301 0.1274 0.1301] Zoom
  (Variables|Default|SetTargetCameraZoom (Math|Float|Clamp(Float) (+ (* Step (Variables|Default|GetZoomSensitivity)) (Variables|Default|GetTargetCameraZoom)) (Variables|Default|GetMinCameraDistance) (Variables|Default|GetMaxCameraDistance))))

(event Custom|RotateCamera
  (params (AxisValue :type Float%20%28double-precision%29) (IsGamepad :type Boolean))
  (bind _returnvalue (Transformation|GetActorRotation))
  (bind (_roll _pitch) (Math|Rotator|BreakRotator _returnvalue))
  ;[0.1301 0.1274 0.1301] Rotate
  (bind _output_get (Variables|Default|SetCurrentYaw (+ (Variables|Default|GetCurrentYaw) (* (Utilities|Time|GetWorldDeltaSeconds) (* (select IsGamepad (Variables|Default|GetRotationSpeedGamepad) (Variables|Default|GetRotationSpeedMouse)) AxisValue)))))
  (Transformation|SetActorRotation (Math|Rotator|MakeRotator _roll _pitch _output_get)))

(event Custom|UseCard
  (params (Slot :type Integer))
  ;[0.1301 0.1274 0.1301] Use_Card
  (Development|PrintString (Utilities|String|Append "Card_" (Utilities|String|ToString(Integer) Slot))))

(event Custom|StartFocus
  (params (TargetActor :type Actor%20Object%20Reference))
  ;[0.1301 0.1274 0.1301] Focus
  (Game|Player|SetViewTargetwithBlend (Game|GetPlayerController 0) TargetActor 0.5 "VTBlend_Linear" 0.0 true))

(event Custom|EndFocus
  ;[0.1301 0.1274 0.1301] Focus
  (Game|Player|SetViewTargetwithBlend (Game|GetPlayerController 0) (Game|Player|GetPlayerPawn 0) 0.5 "VTBlend_Linear" 0.0 true))

(event EventTick
  (params (DeltaSeconds :type Float%20%28single-precision%29))
  (bind _springarm (Variables|Default|GetSpringArm))
  ;[0.1301 0.1274 0.1301] Плавное изменение камеры и расчет скорости пермещения (Tick)
  (Utilities|FlowControl|Sequence
    (:then_1
      (bind _output_get (Variables|/Script/Engine.SpringArmComponent|SetTargetArmLength _springarm (Math|Interpolation|FInterpTo (Variables|/Script/Engine.SpringArmComponent|GetTargetArmLength _springarm) (Variables|Default|GetTargetCameraZoom) DeltaSeconds (Variables|Default|GetInterpSpeed))))
      (Variables|Default|SetCurrentMoveSpeed (/ (Math|Float|Lerp (Variables|Default|GetMinMoveSpeed) (Variables|Default|GetMaxMoveSpeed) (/ (- _output_get (Variables|Default|GetMinCameraDistance)) (- (Variables|Default|GetMaxCameraDistance) (Variables|Default|GetMinCameraDistance)))) (Variables|Default|GetMaxMoveSpeed)))
      (Variables|Default|SetCurrentGamepadTraceRadius (Math|Float|Lerp (Variables|Default|GetMinGamepadTraceRadius) (Variables|Default|GetMaxGamepadTraceRadius) (/ (- _output_get (Variables|Default|GetMinCameraDistance)) (- (Variables|Default|GetMaxCameraDistance) (Variables|Default|GetMinCameraDistance))))))))

(event EventMove
  (params (Direction :type Vector%202D%20Structure))
  (bind (_x _y) (Math|Vector2D|BreakVector2D Direction))
  ;[0.1301 0.1274 0.1301] Movement
  (Pawn|Input|AddMovementInput (Math|Vector|Normalize (+ (* (Transformation|GetActorForwardVector) _x) (* (Transformation|GetActorRightVector) _y))) (Variables|Default|GetCurrentMoveSpeed) false))

(fn ConstructionScript)

(fn SetCameraFocusedState
  (params (TagetActor :type Actor%20Object%20Reference))
  (Transformation|SetActorLocation (Math|Interpolation|VInterpTo (Transformation|GetActorLocation) (Transformation|GetActorLocation TagetActor) 0.0 5.0) false false))

(fn RestoreCameraState
  (Transformation|SetActorRotation "0, 0, 0")
  (Variables|Default|SetTargetCameraZoom 0.0))

(fn GetGamepadTraceRadius
  (return (Variables|Default|GetCurrentGamepadTraceRadius)))
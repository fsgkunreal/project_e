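; BP_ForceBorder is a throwable-related border effect that drives a Niagara system's Progress parameter from a timeline started on BeginPlay.
; The construction script rebuilds an open spline from 32 points at a fixed radius in the local XY plane.
; Its angle math multiplies degrees by 180/π instead of π/180, so the points do not step evenly around the circle.
; The GrowSpeed play-rate call is disconnected and never runs.
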(event EventBeginPlay
  (bind _progress (Timeline|Timeline PlayFromStart)
    (:Update
      (Niagara|SetNiagaraVariable(Float) (Variables|Default|GetNiagara) "Progress" _progress))))

(fn ConstructionScript
  (bind _spline (Variables|Default|GetSpline))
  (Utilities|FlowControl|Sequence
    (:then_0
      (Spline|ClearSplinePoints _spline true)
      (for _index (range 0 31)
        (Spline|AddSplinePoint _spline (Math|Vector|MakeVector (* (Math|Trig|Cos(Radians) (* (* (/ (Math|Conversions|ToFloat(Integer) _index) 31.0) 3.6e+02) (/ 1.8e+02 (Math|Float|MultiplybyPi 1.0)))) 48.0) (* (Math|Trig|Sin(Radians) (* (* (/ (Math|Conversions|ToFloat(Integer) _index) 31.0) 3.6e+02) (/ 1.8e+02 (Math|Float|MultiplybyPi 1.0)))) 48.0) 0.0) "Local" true))
      (Spline|SetClosedLoop _spline false true))))
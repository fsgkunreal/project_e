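; Interactive physics prop that the player can throw, with outline highlight and interaction availability tied to physics sleep.
; Main action flings it perpendicular to the hit offset, flipped toward pawn forward.
; Holding glides the pawn to it, then shows radius borders and aims by stick or cursor; release throws with distance-scaled force outside a dead zone.
; Hard impacts play impulse-scaled sound and report noise through MakeNoise and ReportNoiseEvent.
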(event OnComponentHit(Mesh)
  (params (HitComponent :type Primitive%20Component%20Object%20Reference) (OtherActor :type Actor%20Object%20Reference) (OtherComp :type Primitive%20Component%20Object%20Reference) (NormalImpulse :type Vector :default "0, 0, 0") (Hit :type Hit%20Result%20Structure%20%28by%20ref%29))
  (bind _location (Collision|BreakHitResult Hit))
  (bind _returnvalue (Math|Vector|VectorLength NormalImpulse))
  (bind _returnvalue_2 (/ _returnvalue 2e+02))
  (bind _returnvalue_3 (Math|Float|Clamp(Float) _returnvalue_2 0.2))
  (bind _returnvalue_4 (* _returnvalue_3 5e+03))
  ;[0.1301 0.1274 0.1301] Доработать
  (if (> _returnvalue 2e+01)
    (Utility|PlayHitSoundwithLoudness _returnvalue)
    (Class|Actor|MakeNoise _returnvalue_4 0 _location _returnvalue_4 "None")
    (Class|AISenseHearing|ReportNoiseEvent _location _returnvalue_4 self _returnvalue_4 "None")))

(event OnComponentSleep(Mesh)
  (params (SleepingComponent :type Primitive%20Component%20Object%20Reference) (BoneName :type Name :default "None"))
  ;[0.1301 0.1274 0.1301] InteractionAvailable / OnHover
  (Variables|Flags|SetbIsInteractionAvailable true))

(event OnComponentWake(Mesh)
  (params (WakingComponent :type Primitive%20Component%20Object%20Reference) (BoneName :type Name :default "None"))
  ;[0.1301 0.1274 0.1301] InteractionAvailable / OnHover
  (Variables|Flags|SetbIsInteractionAvailable false))

(event EventTick
  (params (DeltaSeconds :type Float%20%28single-precision%29))
  (bind _returnvalue (Game|Player|GetPlayerPawn 0))
  (bind _mesh (Variables|Default|GetMesh))
  (bind _returnvalue_2 (Transformation|GetActorLocation _returnvalue))
  (bind _origin (Collision|GetComponentBounds _mesh))
  (bind _returnvalue_3 (Math|Interpolation|VInterpTo _returnvalue_2 _origin DeltaSeconds 4.0))
  ;[0.1301 0.1274 0.1301] Event Tick - Move Pawn to Object
  (if (Variables|Flags|GetbIsMoveToObject)
    (Transformation|SetActorLocation (Game|Player|GetPlayerPawn 0) _returnvalue_3 false false)
    (if (< (Math|Vector|Distance(Vector) _returnvalue_3 _origin) 1.0)
      (Utility|MovetoObject false false))))

(event EventOnHoverEnd
  ;[0.1301 0.1274 0.1301] InteractionAvailable / OnHover
  (Utility|ApplyOutlineEffect false))

(event EventOnHoverStart
  ;[0.1301 0.1274 0.1301] InteractionAvailable / OnHover
  (Utility|ApplyOutlineEffect true))

(event EventDoMainAction
  (params (HitResult :type Hit%20Result%20Structure))
  ;[0.1301 0.1274 0.1301] Throwable
  (Throw|ThrowQuick HitResult))

(event EventDoMainActionHoldReset
  ;[0.1301 0.1274 0.1301] Throwable
  (Utilities|FlowControl|Sequence
    (:then_0
      (Utilities|FlowControl|DoOnce false) ; enters at Reset
    )
    (:then_1
      (Utilities|FlowControl|DoOnce false) ; enters at Reset
    )
    (:then_2
      (Utility|MovetoObject false true)
      (Throw|ThrowExact)
      (for _array_element (Variables|Reference|GetForceBorderReference)
        (Actor|DestroyActor _array_element)
        (Actor|DestroyActor (Variables|Reference|GetInteractiveBorderReference))
        (Components|Activation|SetActive (Variables|Default|GetNiagara) false false)
        (CallFunction|InputActionSetting true true true true)))))

(event EventDoMainActionHold
  (params (HoldTime :type Float%20%28double-precision%29) (Direction :type Vector%202D%20Structure))
  ;[0.1301 0.1274 0.1301] Throwable
  (Utilities|FlowControl|Sequence
    (:then_0
      (Utilities|FlowControl|DoOnce false
        (:Completed
          (Utility|MovetoObject true false))))
    (:then_1
      (if (not (Variables|Flags|GetbIsMoveToObject))
        (Utilities|FlowControl|Sequence
          (:then_0
            (ForceSelector|DrawForceLine Direction))
          (:then_1
            (Utilities|FlowControl|DoOnce false
              (:Completed
                (CallFunction|InputActionSetting false true false false)
                (ForceSelector|SpawnInteractiveBorder)
                (ForceSelector|SpawnForceBorder false)
                (ForceSelector|SpawnForceBorder true)
                (Components|Activation|SetActive (Variables|Default|GetNiagara) true false)))))))))

(fn ConstructionScript
  (bind _staticmesh (Variables|SettingUp|GetStaticMesh))
  (bind _physicalmaterial (Variables|SettingUp|GetPhysicalMaterial))
  (Utilities|FlowControl|Sequence
    (:then_0
      (Utilities|IsValid _staticmesh
        (:Is%20Valid
          (Components|StaticMesh|SetStaticMesh (Variables|Default|GetMesh) _staticmesh))))
    (:then_1
      (Utilities|IsValid _physicalmaterial
        (:Is%20Valid
          (Class|PrimitiveComponent|SetPhysMaterialOverride (Variables|Default|GetMesh) _physicalmaterial))))
    (:then_2
      (Audio|Components|Audio|SetSound (Variables|Default|GetHitSoundComponent) (Variables|SettingUp|GetHitSound)))))

(fn ThrowQuick
  (params (HitResult :type Hit%20Result%20Structure))
  (bind _returnvalue (Transformation|GetActorLocation))
  (bind _impactpoint (Collision|BreakHitResult HitResult))
  (bind _returnvalue_2 (Math|Vector|MakeVector 0.0 0.0 1.0))
  (bind _mesh (Variables|Default|GetMesh))
  (bind _baseforce (Variables|SettingUp|GetBaseForce))
  (bind _liftforce (Variables|SettingUp|GetLiftForce))
  (bind _returnvalue_3 (- _returnvalue _impactpoint))
  (bind _returnvalue_4 (Math|Vector|Normalize _returnvalue_3))
  (bind _returnvalue_5 (Math|Vector|CrossProduct _returnvalue_4 _returnvalue_2))
  (bind _returnvalue_6 (Math|Vector|Normalize _returnvalue_5))
  (bind _updateddirection (Utility|DirectionfromCamera _returnvalue_6))
  (bind _returnvalue_7 (* _updateddirection _baseforce 1.0))
  (bind _returnvalue_8 (Math|Vector|MakeVector (.x _returnvalue_7) (.y _returnvalue_7) _liftforce))
  (Class|PrimitiveComponent|AddAngularImpulseinDegrees _mesh (* _returnvalue_8 "2.000000,2.000000,0.000000") "None" true)
  (Physics|AddImpulse _mesh _returnvalue_8 "None" true))

(fn DirectionfromCamera
  (params (Direction :type Vector))
  (bind _returnvalue (Game|Player|GetPlayerPawn 0))
  (bind _returnvalue_2 (Transformation|GetActorForwardVector _returnvalue))
  (if (< (Math|Vector|DotProduct Direction (Math|Vector|Normalize (Math|Vector|MakeVector (.x _returnvalue_2) (.y _returnvalue_2) 0.0))) 0.0)
    (return (Math|Vector|NegateVector Direction))
    (else
      (return Direction))))

(fn PlayHitSoundwithLoudness
  (params (ImpulseMagnitude :type Float%20%28double-precision%29))
  (bind _hitsoundcomponent (Variables|Default|GetHitSoundComponent))
  (Audio|Components|Audio|SetVolumeMultiplier _hitsoundcomponent (Math|Float|Clamp(Float) (/ ImpulseMagnitude 2.5e+02) 0.1) :!class /Script/Engine.AudioComponent)
  (Audio|Components|Audio|Play _hitsoundcomponent 0.0))

(fn SpawnInteractiveBorder
  (bind _returnvalue (Game|SpawnActorfromClass "/Game/content_0/base/throwable/BP_InteractiveBorder.BP_InteractiveBorder_C" (Math|Conversions|ToTransform(Vector) (.Origin (Collision|GetComponentBounds (Variables|Default|GetMesh)))) "Undefined" "MultiplyWithRoot" 0 0))
  (Variables|Reference|SetInteractiveBorderReference _returnvalue))

(fn SpawnForceBorder
  (params (bIsInnerBorder :type Boolean))
  (bind _returnvalue (Game|SpawnActorfromClass "/Game/content_2/SplineVFX/_GenericSource/BP/BP_ForceBorder.BP_ForceBorder_C" (Math|Transform|MakeTransform (.Origin (Collision|GetComponentBounds (Variables|Default|GetMesh))) "0, 0, 0" (ForceSelector|ApplyDeadZoneRadius bIsInnerBorder)) "Undefined" "MultiplyWithRoot" 0 0))
  (Utilities|Array|Add (Variables|Reference|GetForceBorderReference) _returnvalue))

(fn DrawForceLine
  (params (Direction :type Vector%202D%20Structure))
  (bind _returnvalue (Game|Player|GetPlayerPawn 0))
  (bind _mesh (Variables|Default|GetMesh))
  (bind (_x _y) (Math|Vector2D|BreakVector2D Direction))
  (bind _origin (Collision|GetComponentBounds _mesh))
  (bind _bisgamepad (Utility|GetControlLayout))
  (if _bisgamepad
    (LocalVariables|SetInpactPoint (+ (.Origin (Collision|GetComponentBounds (Variables|Default|GetMesh))) (* (Math|Vector|Normalize (+ (* _x (Transformation|GetActorRightVector _returnvalue)) (* (Transformation|GetActorForwardVector _returnvalue) _y))) (* (Variables|SettingUp|GetSlectorRadius) (Math|Vector2D|Vector2DLength Direction)))))
    (else
      (LocalVariables|SetInpactPoint (.ImpactPoint (Collision|BreakHitResult (.HitResult (Game|Player|GetHitResultUnderCursorbyChannel (Game|GetPlayerController 0) "TraceTypeQuery3" true)))))))
  (if (>= (Math|Vector|VectorLength (- (LocalVariables|GetInpactPoint) _origin)) (Variables|SettingUp|GetSlectorRadius))
    (LocalVariables|SetEndPoint (+ _origin (* (Math|Vector|GetUnitDirection(Vector) _origin (LocalVariables|GetInpactPoint)) (Variables|SettingUp|GetSlectorRadius))))
    (else
      (LocalVariables|SetEndPoint (LocalVariables|GetInpactPoint))))
  (Transformation|SetWorldLocation (Variables|Default|GetSpline) (LocalVariables|GetEndPoint) false false)
  (Variables|Temporary|SetTrhowDirection (- (LocalVariables|GetEndPoint) _origin))
  (Variables|Temporary|SetForceCoefficient%20 (Math|Float|Clamp(Float) (/ (Math|Vector|VectorLength (- (LocalVariables|GetEndPoint) _origin)) (Variables|SettingUp|GetSlectorRadius)))))

(fn ThrowExact
  (bind _mesh (Variables|Default|GetMesh))
  (bind _forcecoefficient_ (Variables|Temporary|GetForceCoefficient%20))
  (bind _trhowdirection (Variables|Temporary|GetTrhowDirection))
  (bind _impulse (Throw|ApplyThrowForce _trhowdirection _forcecoefficient_))
  (if (>= (Variables|Temporary|GetForceCoefficient%20) 0.3)
    (Class|PrimitiveComponent|AddAngularImpulseinDegrees _mesh _impulse "None" true)
    (Physics|AddImpulse _mesh _impulse "None" true)))

(fn ApplyThrowForce
  (params (ThrowDirection :type Vector) (ForceCoefficient%20 :type Float%20%28double-precision%29))
  (bind _returnvalue (Math|Vector|Normalize ThrowDirection))
  (bind _baseforce (Variables|SettingUp|GetBaseForce))
  (bind _baseforce_2 (Variables|SettingUp|GetBaseForce))
  (bind _returnvalue_2 (* ForceCoefficient%20 _baseforce_2))
  (bind _returnvalue_3 (+ _returnvalue_2 _baseforce))
  (bind _returnvalue_4 (* _returnvalue _returnvalue_3))
  (return (Math|Vector|MakeVector (.x _returnvalue_4) (.y _returnvalue_4) (Variables|SettingUp|GetLiftForce))))

(fn ApplyDeadZoneRadius
  (params (bIsDeadZone :type Boolean))
  (bind _slectorradius (Variables|SettingUp|GetSlectorRadius))
  (bind _slectorradius_2 (Variables|SettingUp|GetSlectorRadius))
  (bind _returnvalue (* _slectorradius 0.003))
  (bind _returnvalue_2 (* _slectorradius_2 0.02))
  (if bIsDeadZone
    (return (Math|Vector|MakeVector _returnvalue _returnvalue 1.0))
    (else
      (return (Math|Vector|MakeVector _returnvalue_2 _returnvalue_2 1.0)))))

(fn ApplyOutlineEffect
  (params (bIsHoverStart :type Boolean))
  (if bIsHoverStart
    (if (Variables|Flags|GetbIsInteractionAvailable)
      (Rendering|Material|SetOverlayMaterial (Variables|Default|GetMesh) (Variables|Reference|GetOverlayMaterial) :!class /Script/Engine.MeshComponent))
    (else
      (Rendering|Material|SetOverlayMaterial (Variables|Default|GetMesh) 0 :!class /Script/Engine.MeshComponent))))

(fn SetMousePosition
  (bind _returnvalue (Viewport|GetViewportSize))
  (bind (_x _y) (Math|Vector2D|BreakVector2D _returnvalue))
  (Class|PlayerController|SetMouseLocation (Game|GetPlayerController 0) (Math|Float|Truncate (/ _x 2.0)) (Math|Float|Truncate (/ _y 2.0))))

(fn MovetoObject
  (params (bIsMoveToObject :type Boolean) (bIsHoldReset :type Boolean))
  (bind _bisgamepad (Utility|GetControlLayout))
  (if _bisgamepad
    _
    (else
      (Variables|/Script/Engine.PlayerController|SetbShowMouseCursor (Game|GetPlayerController 0) bIsHoldReset)
      (Utility|SetMousePosition)))
  (Variables|Flags|SetbIsMoveToObject bIsMoveToObject))

(fn GetControlLayout
  (bind _asmy_game_instance (Utilities|Casting|CastToMyGameInstance (Game|GetGameInstance)))
  (switch Utilities|FlowControl|Switch|SwitchonE_ControlLayout (Default|GetControlLayout _asmy_game_instance)
    (:NewEnumerator0
      _)
    (:NewEnumerator1
      _)
    (:NewEnumerator2
      (return true)))
  (return false))

(fn InputActionSetting
  (params (Movement :type Boolean) (Zoom :type Boolean) (Rotate :type Boolean) (TraceInteraction :type Boolean))
  (bind _asbp_controller_base (Utilities|Casting|CastToBP_Controller_Base (Game|GetPlayerController 0)))
  (Default|InputActionSetting _asbp_controller_base Movement Zoom Rotate TraceInteraction))

(fn IsFocusAvailable
  (return false))

(fn IsInteractionAvailable
  (return (Variables|Flags|GetbIsInteractionAvailable)))

(fn IsMainActionAvailable
  (return true))

(fn IsMainHoldActionAvailable
  (return true))

(fn IsSecondActionAvailable
  (return true))

(fn IsSecondHoldActionAvailable
  (return false))
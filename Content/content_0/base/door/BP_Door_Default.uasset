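; Interactable door that players swing open or closed, or drag by hand, with lock status and hover highlight.
; Main and second actions choose direction from the player's side, then interpolate yaw on Tick; locked or end-of-travel attempts play a Timeline nudge.
; Holding projects input, relative to the pawn, onto the door to rotate it.
; When locked, holding blends to an inner or outer handle camera and accumulates progress until unlocked.
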(event EventOnHoverStart
  (bind _door (Variables|Default|GetDoor))
  (if (Variables|Default|GetbIsHandleLocekd)
    (Rendering|Material|SetOverlayMaterial _door "/Game/content_0/interfaces/M_Overlay_RED.M_Overlay_RED" :!class /Script/Engine.MeshComponent)
    (else
      (Rendering|Material|SetOverlayMaterial _door "/Game/content_0/interfaces/M_Overlay_Orange.M_Overlay_Orange" :!class /Script/Engine.MeshComponent))))

(event EventOnHoverEnd
  (Rendering|Material|SetOverlayMaterial (Variables|Default|GetDoor) 0 :!class /Script/Engine.MeshComponent))

(event EventDoMainAction
  (params (HitResult :type Hit%20Result%20Structure))
  ;[0.1301 0.1274 0.1301] Main/Second Action
  (if (Variables|Default|GetbIsAnaimation)
    (CallFunction|InterpSpeedSetting false true false)
    (else
      (bind (_rotationblocked _temprotationangleb _temprotationanglea) (CallFunction|DetermineDirection true (Variables|Default|GetbIsHandleLocekd)))
      (if _rotationblocked
        (Variables|Default|SetTempRotationAngleB _temprotationangleb)
        (Variables|Default|SetTempRotationAngleA _temprotationanglea)
        (bind _open (Timeline|Timeline PlayFromStart)
          (:Update
            (Transformation|SetRelativeRotation (Variables|Default|GetDoor) (Math|Rotator|MakeRotator 0.0 0.0 (Math|Float|Lerp (Variables|Default|GetTempRotationAngleA) (Variables|Default|GetTempRotationAngleB) _open)) false false)
            (Audio|Components|Audio|Play (Variables|Default|GetAudio) 0.0)))
        (else
          (Utilities|AnimationHandler true false))))))

(event EventDoMainActionHold
  (params (HoldTime :type Float%20%28double-precision%29) (Direction :type Vector%202D%20Structure))
  ;[0.1301 0.1274 0.1301] MainActionHold
  (if (Variables|Default|GetbIsHandleLocekd)
    (Utilities|FlowControl|Sequence
      (:then_0
        (Utilities|FlowControl|DoOnce false
          (:Completed
            (CallFunction|SwitchView true))))
      (:then_1
        (CallFunction|HandleInteraction Direction)))
    (else
      (CallFunction|DoorInteraction Direction))))

(event EventDoMainActionHoldReset
  ;[0.1301 0.1274 0.1301] MainActionHold
  (Utilities|FlowControl|Sequence
    (:then_0
      (if (Variables|Default|GetbIsHandleLocekd)
        (CallFunction|SwitchView false)))
    (:then_1
      (Utilities|FlowControl|DoOnce false) ; enters at Reset
    )))

(event EventDoSecondAction
  ;[0.1301 0.1274 0.1301] Main/Second Action
  (if (Variables|Default|GetbIsAnaimation)
    (CallFunction|InterpSpeedSetting false true false)
    (else
      (bind (_rotationblocked _temprotationangleb _temprotationanglea) (CallFunction|DetermineDirection false (Variables|Default|GetbIsHandleLocekd)))
      (if _rotationblocked
        (Variables|Default|SetTempRotationAngleB _temprotationangleb)
        (Variables|Default|SetTempRotationAngleA _temprotationanglea)
        (bind _open (Timeline|Timeline PlayFromStart)
          (:Update
            (Transformation|SetRelativeRotation (Variables|Default|GetDoor) (Math|Rotator|MakeRotator 0.0 0.0 (Math|Float|Lerp (Variables|Default|GetTempRotationAngleA) (Variables|Default|GetTempRotationAngleB) _open)) false false)
            (Audio|Components|Audio|Play (Variables|Default|GetAudio) 0.0)))
        (else
          (Utilities|AnimationHandler true false))))))

(event EventTick
  (params (DeltaSeconds :type Float%20%28single-precision%29))
  ;[0.1301 0.1274 0.1301] EventTick
  (Utilities|FlowControl|Sequence
    (:then_0
      (if (Variables|Default|GetbIsAnaimation)
        (Utilities|FlowControl|Sequence
          (:then_0
            (bind _output_get (Variables|Default|SetRotationAngle (Math|Interpolation|FInterpTo (.yaw (Variables|/Script/Engine.SceneComponent|GetRelativeRotation (Variables|Default|GetDoor))) (Variables|Default|GetTempRotationAngle) DeltaSeconds (Variables|Default|GetInterpSpeed))))
            (Transformation|SetRelativeRotation (Variables|Default|GetDoor) (Math|Rotator|MakeRotator 0.0 0.0 _output_get) false false))
          (:then_1
            (Utilities|AnimationHandler false false
              (:Out
                (CallFunction|InterpSpeedSetting true false false)))))))
    (:then_1
      (if (Variables|Default|GetbIsHandleLocekd)
        (CallFunction|SetStatus "(TagName=\"Door.Status.Locked\")")
        (elif (> (Variables|Default|GetRotationAngle) (Variables|Default|GetMinRotationAngle))
          (CallFunction|SetStatus "(TagName=\"Door.Status.Open\")")
          (else
            (CallFunction|SetStatus "(TagName=\"Door.Status.Closed\")")))))))

(fn ConstructionScript)

(fn HandleInteraction
  (params (Direction :type Vector%202D%20Structure))
  (bind _door (Variables|Default|GetDoor))
  (bind _origin (Collision|GetComponentBounds _door))
  (if (<= (Variables|Default|GetHandleProgress) 9.5)
    (Rendering|Debug|DrawDebugSphere _origin 1e+01 12 "(R=1.000000,G=1.000000,B=1.000000,A=1.000000)" 0.0)
    (bind _output_get (Variables|Default|SetHandleProgress (Math|Float|Clamp(Float) (+ (* (Math|Vector2D|Vector2DLength Direction) 0.25) (Variables|Default|GetHandleProgress)) 0.0 1e+01)))
    (Rendering|Debug|DrawDebugSphere _origin _output_get 12 "(R=1.000000,G=0.000000,B=0.000000,A=1.000000)" 0.0)
    (else
      (Variables|Default|SetbIsHandleLocekd false)
      (CallFunction|SwitchView false))))

(fn DoorInteraction
  (params (Direction :type Vector%202D%20Structure))
  (bind _returnvalue (Game|Player|GetPlayerPawn 0))
  (bind _output_get (Variables|Default|SetRotationAngle (Math|Float|Clamp(Float) (+ (* (Math|Vector|DotProduct (Math|Vector|Normalize (+ (* (.x Direction) (Transformation|GetActorRightVector _returnvalue)) (Math|Vector|NegateVector (* (Transformation|GetActorForwardVector _returnvalue) (.y Direction))))) (Math|Vector|GetRightVector (Variables|Default|GetDoor))) (Math|Vector2D|Vector2DLength Direction) 5.0) (Variables|Default|GetRotationAngle)) (Variables|Default|GetMinRotationAngle) (Variables|Default|GetMaxRotationAngle))))
  (Transformation|SetRelativeRotation (Variables|Default|GetDoor) (Math|Rotator|MakeRotator 0.0 0.0 _output_get) false false))

(fn SwitchView
  (params (bIsHandleView :type Boolean))
  (Components|Activation|Deactivate (Variables|Default|GetInnerCamera))
  (Components|Activation|Deactivate (Variables|Default|GetOuterCamera))
  (bind _asbp_controller_base (Utilities|Casting|CastToBP_Controller_Base (Game|GetPlayerController 0)))
  (LocalVariables|SetController _asbp_controller_base)
  (if bIsHandleView
    (if (Utilities|FindInnerSide)
      (Components|Activation|Activate (Variables|Default|GetInnerCamera) false)
      (else
        (Components|Activation|Activate (Variables|Default|GetOuterCamera) false)))
    (Game|Player|SetViewTargetwithBlend (LocalVariables|GetController) self 0.3 "VTBlend_Cubic" 0.3 true)
    (Default|InputActionSetting (LocalVariables|GetController) false false false)
    (else
      (Game|Player|SetViewTargetwithBlend (LocalVariables|GetController) (Game|Player|GetPlayerPawn 0) 0.3 "VTBlend_Cubic" 0.3 true)
      (Default|InputActionSetting (LocalVariables|GetController) true true true))))

(fn DetermineDirection
  (params (bIsMainAction :type Boolean) (bIsHandleLocked :type Boolean))
  (bind _rotationangle (Variables|Default|GetRotationAngle))
  (bind _maxangleforblocked (LocalVariables|GetMaxAngleForBlocked))
  (bind _returnvalue (> _rotationangle _maxangleforblocked))
  (if bIsHandleLocked
    (if bIsMainAction
      (if (Utilities|FindInnerSide)
        (return true -1.5 0.0)
        (else
          (return true 1.5 0.0)))
      (elif (Utilities|FindInnerSide)
        (return true 1.5 0.0)
        (else
          (return true -1.5 0.0))))
    (elif bIsMainAction
      (if (Utilities|FindInnerSide)
        (if (< (Variables|Default|GetRotationAngle) (LocalVariables|GetMinAngleForBlocked))
          (return true (LocalVariables|GetEndAngleForClosedBlockedDoor) 0.0)
          (else
            (bind _output_get (Variables|Default|SetTempRotationAngle (Variables|Default|GetMinRotationAngle)))
            (return false _output_get 0.0)))
        (elif _returnvalue
          (return true (LocalVariables|GetEndAngleForOpenedBlockedDoor) (Variables|Default|GetMaxRotationAngle))
          (else
            (bind _output_get_2 (Variables|Default|SetTempRotationAngle (Variables|Default|GetMaxRotationAngle)))
            (return false _output_get_2 0.0))))
      (elif (Utilities|FindInnerSide)
        (if _returnvalue
          (return true (LocalVariables|GetEndAngleForOpenedBlockedDoor) (Variables|Default|GetMaxRotationAngle))
          (else
            (bind _output_get_3 (Variables|Default|SetTempRotationAngle (Variables|Default|GetMaxRotationAngle)))
            (return false _output_get_3 0.0)))
        (elif (< (Variables|Default|GetRotationAngle) (LocalVariables|GetMinAngleForBlocked))
          (return true (LocalVariables|GetEndAngleForClosedBlockedDoor) 0.0)
          (else
            (bind _output_get_4 (Variables|Default|SetTempRotationAngle (Variables|Default|GetMinRotationAngle)))
            (return false _output_get_4 0.0)))))))

(fn InterpSpeedSetting
  (params (Restore :type Boolean) (Reduce :type Boolean) (MultiplyReduce :type Boolean))
  (Utilities|FlowControl|Sequence
    (:then_0
      (if Restore
        (Variables|Default|SetInterpSpeed (LocalVariables|GetBaseSpeed))))
    (:then_1
      (if Reduce
        (if MultiplyReduce
          (Variables|Default|SetInterpSpeed (* (Variables|Default|GetInterpSpeed) (LocalVariables|GetBaseReduce)))
          (elif (== (Variables|Default|GetInterpSpeed) (LocalVariables|GetBaseSpeed))
            (Variables|Default|SetInterpSpeed (* (Variables|Default|GetInterpSpeed) (LocalVariables|GetBaseReduce)))))))))

(fn IsFocusAvailable
  (return false))

(fn IsInteractionAvailable
  (return true))

(fn IsMainActionAvailable
  (return true))

(fn IsMainHoldActionAvailable
  (return true))

(fn IsSecondActionAvailable
  (return true))

(fn IsSecondHoldActionAvailable
  (return true))
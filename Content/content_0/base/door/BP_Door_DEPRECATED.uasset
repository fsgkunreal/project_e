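; Deprecated interactable door that highlights on hover, toggles open or closed on the main action, and swings with held directional input.
; The toggle uses a timeline, while holding projects player-relative input onto the door to drive its clamped yaw.
; While OnClock is set, holding instead blends to the inner or outer camera by viewer side and fills a debug-sphere progress at that handle, clearing OnClock and restoring the view when full.
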(event Custom|OnHoverStart_1_1
  (Rendering|Material|SetOverlayMaterial (Variables|Default|GetDoor) "/Game/content_0/interfaces/M_Overlay.M_Overlay" :!class /Script/Engine.MeshComponent)
  (Development|PrintString "HoverStart"))

(event EventDoMainActionHold
  (params (HoldTime :type Float%20%28double-precision%29) (Direction :type Vector%202D%20Structure))
  (bind _returnvalue (Game|Player|GetPlayerPawn 0))
  (Variables|Default|SetDirection Direction)
  (if (Variables|Default|GetbOnClock)
    (Utilities|FlowControl|Sequence
      (:then_0
        (Utilities|FlowControl|DoOnce false
          (:Completed
            (CallFunction|SetViewTraget true))))
      (:then_1
        (CallFunction|HandleInteraction)))
    (else
      (bind _output_get (Variables|Default|SetDeltaYaw (Math|Float|Clamp(Float) (+ (* (Math|Vector|DotProduct (Math|Vector|Normalize (+ (* (.x (Variables|Default|GetDirection)) (Transformation|GetActorRightVector _returnvalue)) (Math|Vector|NegateVector (* (Transformation|GetActorForwardVector _returnvalue) (.y (Variables|Default|GetDirection)))))) (Transformation|GetActorRightVector)) (Class|KismetMathLibrary|VSize2DSquared (Variables|Default|GetDirection)) 5.0) (Variables|Default|GetDeltaYaw)) 0.0 105.0)))
      (Transformation|SetRelativeRotation (Variables|Default|GetDoor) (Math|Rotator|MakeRotator 0.0 0.0 _output_get) false false))))

(event EventDoMainAction
  (params (HitResult :type Hit%20Result%20Structure))
  (if (not (Variables|Default|GetbOnClock))
    (bind _currentrotation (CallFunction|FlipRotation))
    (bind _open (Timeline|Timeline PlayFromStart)
      (:Update
        (bind _output_get (Variables|Default|SetDeltaYaw (Math|Float|Lerp (.yaw (Variables|/Script/Engine.SceneComponent|GetRelativeRotation (Variables|Default|GetDoor))) _currentrotation _open)))
        (Transformation|SetRelativeRotation (Variables|Default|GetDoor) (Math|Rotator|MakeRotator 0.0 0.0 _output_get) false false)))))

(event EventOnHoverEnd
  (Rendering|Material|SetOverlayMaterial (Variables|Default|GetDoor) 0 :!class /Script/Engine.MeshComponent)
  (Development|PrintString "HoverEnd"))

(event EventTick
  (params (DeltaSeconds :type Float%20%28single-precision%29))
  (Utilities|FlowControl|Sequence
    (:then_0
      (if (> (.yaw (Variables|/Script/Engine.SceneComponent|GetRelativeRotation (Variables|Default|GetDoor))) 52.5)
        (Variables|Default|SetbIsOpen true)
        (else
          (Variables|Default|SetbIsOpen false))))))

(event EventDoMainActionHoldReset
  (Utilities|FlowControl|Sequence
    (:then_0
      (if (Variables|Default|GetbOnClock)
        (CallFunction|SetViewTraget false)))
    (:then_1
      (Utilities|FlowControl|DoOnce false) ; enters at Reset
    )))

(fn ConstructionScript)

(fn FlipRotation
  (if (Variables|Default|GetbIsOpen)
    (return 0.0)
    (else
      (return 105.0))))

(fn CheckonClock
  (bind _asbp_controller_base (Utilities|Casting|CastToBP_Controller_Base (Game|GetPlayerController 0))))

(fn SetViewTraget
  (params (bIsActorView :type Boolean))
  (bind _asbp_controller_base (Utilities|Casting|CastToBP_Controller_Base (Game|GetPlayerController 0)))
  (LocalVariables|SetController _asbp_controller_base)
  (if bIsActorView
    (if (> (Math|Vector|DotProduct (Transformation|GetActorForwardVector) (Math|Vector|Normalize (- (Transformation|GetActorLocation (Game|GetPlayerCameraManager 0)) (Transformation|GetActorLocation)))) 0.0)
      (Components|Activation|Activate (Variables|Default|GetCameraInner) false)
      (else
        (Components|Activation|Activate (Variables|Default|GetCamera) false)))
    (Game|Player|SetViewTargetwithBlend (LocalVariables|GetController) self 0.3 "VTBlend_Cubic" 0.3 true)
    (else
      (Game|Player|SetViewTargetwithBlend (LocalVariables|GetController) (Game|Player|GetPlayerPawn 0) 0.3 "VTBlend_Cubic" 0.3 true)
      (Components|Activation|Deactivate (Variables|Default|GetCameraInner))
      (Components|Activation|Deactivate (Variables|Default|GetCamera)))))

(fn HandleInteraction
  (if (<= (Variables|Default|GetProgress) 9.0)
    (if (> (Math|Vector|DotProduct (Transformation|GetActorForwardVector) (Math|Vector|Normalize (- (Transformation|GetActorLocation (Game|GetPlayerCameraManager 0)) (Transformation|GetActorLocation)))) 0.0)
      (LocalVariables|SetCurrentHand (Variables|Default|GetHand_In))
      (else
        (LocalVariables|SetCurrentHand (Variables|Default|GetHand_Out))))
    (Rendering|Debug|DrawDebugSphere (.Origin (Collision|GetComponentBounds (LocalVariables|GetCurrentHand))) 1e+01 12 "(R=1.000000,G=1.000000,B=1.000000,A=1.000000)" 0.0)
    (bind _output_get (Variables|Default|SetProgress (Math|Float|Clamp(Float) (+ (* (Math|Vector2D|Vector2DLength (Variables|Default|GetDirection)) 0.3) (Variables|Default|GetProgress)) 0.0 1e+01)))
    (Rendering|Debug|DrawDebugSphere (.Origin (Collision|GetComponentBounds (LocalVariables|GetCurrentHand))) _output_get 12 "(R=0.590619,G=0.045186,B=0.003035,A=1.000000)" 0.0)
    (else
      (Variables|Default|SetbOnClock false)
      (CallFunction|SetViewTraget false)
      (Variables|Default|SetProgress 0.0))))

(fn IsFocusAvailable
  (return true))

(fn IsInteractionAvailable
  (return true))

(fn IsMainActionAvailable
  (return true))

(fn IsMainHoldActionAvailable
  (return true))

(fn IsSecondActionAvailable
  (return false))

(fn IsSecondHoldActionAvailable
  (return false))

(fn OnHoverStart
  (return))
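; Interactable seal that the player hold-reveals, then hold-unseals for a tier-based reward, currently only printed.
; Gameplay-tag status moves between Hidden, Revealed, Blocked and Completed, with timers driving reveal, expiry and unseal progress from modifier stats.
; Enemy overlap or hover start cancels reveals and temporarily blocks revealed seals.
; Niagara, audio and custom primitive data on the plane show state, with a timeline rewinding cancelled reveal effects.
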(event OnComponentBeginOverlap(EnemyCollision)
  (params (OverlappedComponent :type Primitive%20Component%20Object%20Reference) (OtherActor :type Actor%20Object%20Reference) (OtherComp :type Primitive%20Component%20Object%20Reference) (OtherBodyIndex :type Integer) (bFromSweep :type Boolean) (SweepResult :type Hit%20Result%20Structure%20%28by%20ref%29))
  ;[0.1301 0.1274 0.1301] Blocked
  (if (Actor|ActorHasTag OtherActor "Enemy")
    (Block|BlockedStart)
    ;[0.1166 0.1236 0.1458] MainActionHoldReset
    (Reveal|RevealCancel)
    (CallFunction|NiagaraHandler false)
    (bind _reset (Timeline|Timeline PlayFromStart)
      (:Update
        (CallFunction|ResetRevealEffect _reset)))))

(event EventOnHoverStart
  ;[0.1166 0.1236 0.1458] OnHoverStart
  ;[0.1301 0.1274 0.1301] Blocked
  (Block|BlockedStart)
  ;[0.1166 0.1236 0.1458] MainActionHoldReset
  (Reveal|RevealCancel)
  (CallFunction|NiagaraHandler false)
  (bind _reset (Timeline|Timeline PlayFromStart)
    (:Update
      (CallFunction|ResetRevealEffect _reset))))

(event EventOnHoverEnd
  (bind _status (Variables|Default|GetStatus))
  ;[0.1166 0.1236 0.1458] OnHoverEnd
  (if (== (GameplayTags|MakeLiteralGameplayTag "(TagName=\"Seal.Status.Revealed\")") _status)
    (Unseal|UnsealCancel)
    (elif (== _status (GameplayTags|MakeLiteralGameplayTag "(TagName=\"Seal.Status.Hidden\")"))
      _)))

(event EventDoMainActionHoldReset
  (bind _status (Variables|Default|GetStatus))
  ;[0.1166 0.1236 0.1458] MainActionHoldReset
  (if (== (GameplayTags|MakeLiteralGameplayTag "(TagName=\"Seal.Status.Revealed\")") _status)
    (Unseal|UnsealCancel)
    (elif (== _status (GameplayTags|MakeLiteralGameplayTag "(TagName=\"Seal.Status.Hidden\")"))
      (Reveal|RevealCancel)
      (CallFunction|NiagaraHandler false)
      (bind _reset (Timeline|Timeline PlayFromStart)
        (:Update
          (CallFunction|ResetRevealEffect _reset))))))

(event EventDoMainActionHold
  (params (HoldTime :type Float%20%28double-precision%29) (Direction :type Vector%202D%20Structure))
  (bind _status (Variables|Default|GetStatus))
  ;[0.1166 0.1236 0.1458] MainActionHoldReset
  (if (== (GameplayTags|MakeLiteralGameplayTag "(TagName=\"Seal.Status.Revealed\")") _status)
    (Unseal|UnsealStarted)
    (elif (== _status (GameplayTags|MakeLiteralGameplayTag "(TagName=\"Seal.Status.Hidden\")"))
      (Reveal|RevealStarted)
      (Utilities|FlowControl|Sequence
        (:then_0
          (CallFunction|RevealEffect HoldTime))
        (:then_1
          (CallFunction|NiagaraHandler true))))))

(event EventTick
  (params (DeltaSeconds :type Float%20%28single-precision%29)))

(event EventBeginPlay
  ;[0.1301 0.1274 0.1301] BeginPlay
  (Default|SetBaseValue (Variables|Default|GetBP_ModifierManagerComponent) "(TagName=\"Stat.Seal.RevealDuration\")" 5.0)
  (Set|SetStatus "(TagName=\"Seal.Status.Hidden\")"))

(fn ConstructionScript)

(fn GetKey
  (return (Variables|Default|GetKey)))

(fn GetStatus
  (return (Variables|Default|GetStatus)))

(fn GetTier
  (return (Variables|Default|GetTier)))

(fn GetRevealDuration
  (return (Default|GetFinalValue (Variables|Default|GetBP_ModifierManagerComponent) "(TagName=\"Stat.Seal.RevealDuration\")")))

(fn GetRequiredPoints
  (return (Math|Float|Truncate (Default|GetFinalValue (Variables|Default|GetBP_ModifierManagerComponent) "(TagName=\"Stat.Seal.RequiredPoints\")"))))

(fn GetCurrentValue
  (return (Variables|Default|GetCurrentValue)))

(fn GetRewardValue
  (switch Utilities|FlowControl|Switch|SwitchonE_SealTier (Get|GetTier)
    (:NewEnumerator0
      (return 1))
    (:NewEnumerator1
      (return 2))
    (:NewEnumerator2
      (return 3))))

(fn InitializeSealStats)

(fn SetStatus
  (params (NewStatus :type Gameplay%20Tag%20Structure))
  (if (not (== NewStatus (Variables|Default|GetStatus)))
    (bind _output_get (LocalVariables|SetOldStatus (Variables|Default|GetStatus)))
    (bind _output_get_2 (Variables|Default|SetStatus NewStatus))
    (Default|CallOnStatusChanged _output_get_2 _output_get)))

(fn GetWardProgressSpeed
  (bind _outactors (Actor|GetAllActorsOfClass "/Game/content_0/base/ward/BP_Character_Ward.BP_Character_Ward_C"))
  (return (Default|GetFinalValue (Variables|/Game/content_1/scripts/ai/characters/character_base.character_base_C|GetModifierManager (Utilities|Array|Get(acopy) _outactors)) "(TagName=\"Stat.Ward.SealProgressSpeed\")")))

(fn AddRewardtoPlayer
  (params (Value :type Integer))
  (Development|PrintString (Utilities|String|Append "Reward added: " (Utilities|String|ToString(Integer) Value))))

(fn Set)

(fn SetTier
  (params (Tier :type E_SealTier%20Enum :default "NewEnumerator0"))
  (Variables|Default|SetTier Tier))

(fn RevealCompleted
  (if (== (GameplayTags|MakeLiteralGameplayTag "(TagName=\"Seal.Status.Hidden\")") (Variables|Default|GetStatus))
    (Audio|Components|Audio|Play (Variables|Default|GetSealRevealComplete) 0.0)
    (Components|Activation|SetActive (Variables|Default|GetNiagaraRevealCompleted) true false)
    (Set|SetStatus "(TagName=\"Seal.Status.Revealed\")")
    (bind _returnvalue (Utilities|Time|SetTimerbyFunctionName 0 "RevealTimerExpired" 2e+01))
    (Variables|Default|SetRevealTimer _returnvalue)))

(fn RevealTimerExpired
  (if (== (GameplayTags|MakeLiteralGameplayTag "(TagName=\"Seal.Status.Revealed\")") (Variables|Default|GetStatus))
    (Set|SetStatus "(TagName=\"Seal.Status.Hidden\")")
    (Variables|Default|SetCurrentValue 0.0)
    (Utilities|Time|ClearandInvalidateTimerbyHandle (Variables|Default|GetRevealTimer))
    (Audio|Components|Audio|Stop (Variables|Default|GetRevealProccesed))
    (Utilities|FlowControl|Sequence
      (:then_0
        (Audio|Components|Audio|Play (Variables|Default|GetSealRevealCanceled) 0.0))
      (:then_1
        (Rendering|Material|SetCustomPrimitiveDataFloat (Variables|Default|GetPlane) 26 0.0)))))

(fn RevealStarted
  (if (not (Class|KismetSystemLibrary|IsTimerActive 0 "RevealCompleted"))
    (Utilities|Time|SetTimerbyFunctionName 0 "RevealCompleted" (Get|GetRevealDuration) false true)))

(fn RevealCancel
  (if (== (GameplayTags|MakeLiteralGameplayTag "(TagName=\"Seal.Status.Hidden\")") (Variables|Default|GetStatus))
    (Utilities|Time|ClearTimerbyFunctionName 0 "RevealCompleted")))

(fn UnsealStarted
  (if (not (Class|KismetSystemLibrary|IsTimerActive 0 "UnsealProgress"))
    (Utilities|Time|PauseTimerbyHandle (Variables|Default|GetRevealTimer))
    (Utilities|Time|SetTimerbyFunctionName 0 "UnsealProgress" (Utilities|Time|GetWorldDeltaSeconds) true)))

(fn UnsealCancel
  (if (== (GameplayTags|MakeLiteralGameplayTag "(TagName=\"Seal.Status.Revealed\")") (Variables|Default|GetStatus))
    (Utilities|Time|ClearTimerbyFunctionName 0 "UnsealProgress")
    (Utilities|Time|UnpauseTimerbyHandle (Variables|Default|GetRevealTimer))
    (Variables|Default|SetCurrentValue 0.0)))

(fn UnsealProgress
  (bind _output_get (Variables|Default|SetCurrentValue (+ (* (Utilities|Time|GetWorldDeltaSeconds) (Get|GetWardProgressSpeed)) (Variables|Default|GetCurrentValue))))
  (if (>= _output_get (Get|GetRequiredPoints))
    (Utilities|Time|ClearTimerbyFunctionName 0 "UnsealProgress")
    (Unseal|UnsealCompleted)
    (else
      (Development|PrintString (Utilities|String|Append "Progress: " (Utilities|String|ToString(Float) (Variables|Default|GetCurrentValue)) " / " (Utilities|String|ToString(Integer) (Get|GetRequiredPoints))) true true "(R=1.000000,G=0.738652,B=0.000000,A=1.000000)" 2.0 "ProgressUnseal"))))

(fn UnsealCompleted
  (Utilities|Time|ClearandInvalidateTimerbyHandle (Variables|Default|GetRevealTimer))
  (CallFunction|AddRewardtoPlayer (Get|GetRewardValue))
  (Set|SetStatus "(TagName=\"Seal.Status.Completed\")"))

(fn BlockedTimerExpired
  (if (== (Variables|Default|GetStatus) (GameplayTags|MakeLiteralGameplayTag "(TagName=\"Seal.Status.Blocked\")"))
    (Set|SetStatus "(TagName=\"Seal.Status.Hidden\")")
    (Variables|Default|SetCurrentValue 0.0)
    (Utilities|Time|ClearandInvalidateTimerbyHandle (Variables|Default|GetBlockedTimer))
    (Components|Activation|SetActive (Variables|Default|GetNiagaraBlocked) false false)
    (Audio|Components|Audio|Play (Variables|Default|GetSealBlockedStartEnd) 0.0)
    (Audio|Components|Audio|Stop (Variables|Default|GetSealBlockedProccesed))))

(fn BlockedStart
  (if (== (Variables|Default|GetStatus) (GameplayTags|MakeLiteralGameplayTag "(TagName=\"Seal.Status.Revealed\")"))
    (Unseal|UnsealCancel)
    (Utilities|Time|ClearandInvalidateTimerbyHandle (Variables|Default|GetRevealTimer))
    (Set|SetStatus "(TagName=\"Seal.Status.Blocked\")")
    (Components|Activation|SetActive (Variables|Default|GetNiagaraRevealCompleted) false false)
    (Components|Activation|SetActive (Variables|Default|GetNiagaraBlocked) true false)
    (Audio|Components|Audio|Play (Variables|Default|GetSealBlockedStartEnd) 0.0)
    (Audio|Components|Audio|Play (Variables|Default|GetSealBlockedProccesed) 0.0)
    (bind _returnvalue (Utilities|Time|SetTimerbyFunctionName 0 "BlockedTimerExpired" 1e+01))
    (Variables|Default|SetBlockedTimer _returnvalue)))

(fn NiagaraHandler
  (params (bIsActive :type Boolean))
  (Components|Activation|SetActive (Variables|Default|GetNiagaraRevealStarted) bIsActive false))

(fn RevealEffect
  (params (HoldTime :type Float%20%28double-precision%29))
  (if (Audio|Components|Audio|IsPlaying (Variables|Default|GetRevealProccesed))
    _
    (else
      (Audio|Components|Audio|Play (Variables|Default|GetSealRevealStarted) 0.0)
      (Audio|Components|Audio|Play (Variables|Default|GetRevealProccesed) 0.0)))
  (bind _output_get (Variables|Default|SetRevealProgress (Math|Float|Lerp 0.0 1.0 (/ HoldTime (* (Get|GetRevealDuration) 1.75)))))
  (Rendering|Material|SetCustomPrimitiveDataFloat (Variables|Default|GetPlane) 26 _output_get))

(fn ResetRevealEffect
  (params (Alpha :type Float%20%28double-precision%29))
  (if (Audio|Components|Audio|IsPlaying (Variables|Default|GetRevealProccesed))
    (Audio|Components|Audio|Stop (Variables|Default|GetRevealProccesed))
    (Audio|Components|Audio|Play (Variables|Default|GetSealRevealCanceled) 0.0))
  (Rendering|Material|SetCustomPrimitiveDataFloat (Variables|Default|GetPlane) 26 (Math|Float|Lerp 0.0 (Variables|Default|GetRevealProgress) Alpha)))

(fn IsFocusAvailable
  (return false))

(fn IsInteractionAvailable
  (return true))

(fn IsMainActionAvailable
  (return true))

(fn IsMainHoldActionAvailable
  (return true))

(fn IsSecondActionAvailable
  (return false))

(fn IsSecondHoldActionAvailable
  (return false))
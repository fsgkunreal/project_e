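; Interactable seal actor that the player reveals and an AI then unseals, moving through gameplay-tag statuses Hidden, Revealed, Blocked and Completed.
; Holding the main action runs a reveal timer, driving the plane's custom primitive data; completion emits AI noise and starts an expiry timer.
; Second action toggles unsealing, which Tick advances at Ward speed toward a tier-based reward, currently only printed.
; Enemy overlap temporarily blocks a revealed seal before it returns to Hidden.
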(event OnComponentBeginOverlap(EnemyCollision)
  (params (OverlappedComponent :type Primitive%20Component%20Object%20Reference) (OtherActor :type Actor%20Object%20Reference) (OtherComp :type Primitive%20Component%20Object%20Reference) (OtherBodyIndex :type Integer) (bFromSweep :type Boolean) (SweepResult :type Hit%20Result%20Structure%20%28by%20ref%29))
  ;[0.1301 0.1274 0.1301] Blocked
  (if (Actor|ActorHasTag OtherActor "Enemy")
    (Block|BlockedStart)
    ;[0.1166 0.1236 0.1458] MainActionHoldReset
    (Reveal|RevealCancel)
    (CallFunction|NiagaraHandler 0 false)
    (bind _reset (Timeline|Timeline PlayFromStart)
      (:Update
        (CallFunction|ResetRevealEffect _reset)))))

(event Custom|Blocked
  ;[0.1166 0.1236 0.1458] MainActionHoldReset
  (Block|BlockedStart)
  (Reveal|RevealCancel)
  (bind _reset (Timeline|Timeline_0 PlayFromStart)
    (:Update
      (CallFunction|ResetRevealEffect _reset))
    (:Finished
      (Variables|Default|SetRevealProgress 0.0)
      (Variables|Default|SetHoldTime 0.0))))

(event Custom|RevealCancelEvent
  ;[0.1166 0.1236 0.1458] MainActionHoldReset
  (Reveal|RevealCancel)
  (bind _reset (Timeline|Timeline_0 PlayFromStart)
    (:Update
      (CallFunction|ResetRevealEffect _reset))
    (:Finished
      (Variables|Default|SetRevealProgress 0.0)
      (Variables|Default|SetHoldTime 0.0))))

(event EventOnHoverStart
  ;[0.1166 0.1236 0.1458] OnHoverStart
  (Variables|Default|SetbIsOnHover true))

(event EventBeginPlay
  ;[0.1301 0.1274 0.1301] BeginPlay
  (Set|SetStatus "(TagName=\"Seal.Status.Hidden\")"))

(event EventOnHoverEnd
  ;[0.1166 0.1236 0.1458] MainActionHoldReset
  (Variables|Default|SetbIsOnHover false)
  (CallFunction|InputActionSetting true true true true)
  (if (== (Variables|Default|GetStatus) (GameplayTags|MakeLiteralGameplayTag "(TagName=\"Seal.Status.Hidden\")"))
    (Reveal|RevealCancel)
    (bind _reset (Timeline|Timeline_0 PlayFromStart)
      (:Update
        (CallFunction|ResetRevealEffect _reset))
      (:Finished
        (Variables|Default|SetRevealProgress 0.0)
        (Variables|Default|SetHoldTime 0.0)))))

(event EventTick
  (params (DeltaSeconds :type Float%20%28single-precision%29))
  (Unseal|UnsealProgress (Variables|Default|GetbIsAIInteraction)))

(event EventDoSecondAction
  (params (HitResult :type Hit%20Result%20Structure))
  (if (Variables|Default|GetbIsAIInteraction)
    (AI_Interaction|AIUnsealCancel)
    (else
      (AI_Interaction|AIUnsealStart))))

(event EventDoMainActionHold
  (params (HoldTime :type Float%20%28double-precision%29) (Direction :type Vector%202D%20Structure))
  ;[0.1166 0.1236 0.1458] MainActionHold
  (CallFunction|InputActionSetting false true false true)
  (if (== (Variables|Default|GetStatus) (GameplayTags|MakeLiteralGameplayTag "(TagName=\"Seal.Status.Hidden\")"))
    (Reveal|RevealStarted)
    (CallFunction|RevealEffect)))

(event EventDoMainActionHoldReset
  ;[0.1166 0.1236 0.1458] MainActionHoldReset
  (CallFunction|InputActionSetting true true true true)
  (if (== (Variables|Default|GetStatus) (GameplayTags|MakeLiteralGameplayTag "(TagName=\"Seal.Status.Hidden\")"))
    (Reveal|RevealCancel)
    (bind _reset (Timeline|Timeline_0 PlayFromStart)
      (:Update
        (CallFunction|ResetRevealEffect _reset))
      (:Finished
        (Variables|Default|SetRevealProgress 0.0)
        (Variables|Default|SetHoldTime 0.0)))))

(fn ConstructionScript)

(fn GetKey
  (return (Variables|Default|GetKey)))

(fn GetStatus
  (return (Variables|Default|GetStatus)))

(fn GetTier
  (return (Variables|Default|GetTier)))

(fn GetRevealDuration
  (return (Default|GetFinalValue (Variables|Default|GetBP_ModifierManagerComponent) "(TagName=\"Stat.Seal.RevealDuration\")")))

(fn GetRequiredPoints
  (return (Math|Float|Truncate (Default|GetFinalValue (Variables|Default|GetBP_ModifierManagerComponent) "(TagName=\"Stat.Seal.RequiredPoints\")"))))

(fn GetCurrentValue
  (return (Variables|Default|GetCurrentValue)))

(fn GetRewardValue
  (switch Utilities|FlowControl|Switch|SwitchonE_SealTier (Get|GetTier)
    (:NewEnumerator0
      (return 1))
    (:NewEnumerator1
      (return 2))
    (:NewEnumerator2
      (return 3))))

(fn InitializeSealStats)

(fn SetStatus
  (params (NewStatus :type Gameplay%20Tag%20Structure))
  (if (not (== NewStatus (Variables|Default|GetStatus)))
    (bind _output_get (LocalVariables|SetOldStatus (Variables|Default|GetStatus)))
    (bind _output_get_2 (Variables|Default|SetStatus NewStatus))
    (Default|CallOnStatusChanged _output_get_2 _output_get)))

(fn GetWardProgressSpeed
  (bind _outactors (Actor|GetAllActorsOfClass "/Game/content_0/base/ward/BP_Character_Ward.BP_Character_Ward_C"))
  (if (== (Default|GetFinalValue (Variables|/Game/content_1/scripts/ai/characters/character_base.character_base_C|GetModifierManager (Utilities|Array|Get(acopy) _outactors)) "(TagName=\"Stat.Ward.SealProgressSpeed\")") 0.0)
    (return 1.0)
    (else
      (return (Default|GetFinalValue (Variables|/Game/content_1/scripts/ai/characters/character_base.character_base_C|GetModifierManager (Utilities|Array|Get(acopy) _outactors)) "(TagName=\"Stat.Ward.SealProgressSpeed\")")))))

(fn AddRewardtoPlayer
  (params (Value :type Integer))
  (Development|PrintString (Utilities|String|Append "Reward added: " (Utilities|String|ToString(Integer) Value))))

(fn Set)

(fn SetTier
  (params (Tier :type E_SealTier%20Enum :default "NewEnumerator0"))
  (Variables|Default|SetTier Tier))

(fn RevealCompleted
  (if (== (GameplayTags|MakeLiteralGameplayTag "(TagName=\"Seal.Status.Hidden\")") (Variables|Default|GetStatus))
    (CallFunction|Noise "(TagName=\"AI.Environment.Seal.Revealed\")" (Variables|/Script/Engine.AudioComponent|GetSound (Variables|Default|GetSealRevealComplete)) (Transformation|GetActorLocation) 1e+04 self)
    (CallFunction|NiagaraHandler (Variables|Default|GetNiagaraRevealCompleted) true)
    (Set|SetStatus "(TagName=\"Seal.Status.Revealed\")")
    (bind _returnvalue (Utilities|Time|SetTimerbyFunctionName 0 "RevealTimerExpired" 2e+01))
    (Variables|Default|SetRevealTimer _returnvalue)))

(fn RevealTimerExpired
  (if (== (GameplayTags|MakeLiteralGameplayTag "(TagName=\"Seal.Status.Revealed\")") (Variables|Default|GetStatus))
    (Set|SetStatus "(TagName=\"Seal.Status.Hidden\")")
    (Variables|Default|SetCurrentValue 0.0)
    (Utilities|Time|ClearandInvalidateTimerbyHandle (Variables|Default|GetRevealTimer))
    (Audio|Components|Audio|Stop (Variables|Default|GetRevealProccesed))
    (Utilities|FlowControl|Sequence
      (:then_0
        (Audio|Components|Audio|Play (Variables|Default|GetSealRevealCanceled) 0.0))
      (:then_1
        (Rendering|Material|SetCustomPrimitiveDataFloat (Variables|Default|GetPlane) 26 0.0)))))

(fn RevealStarted
  (if (not (Class|KismetSystemLibrary|IsTimerActive 0 "RevealCompleted"))
    (Utilities|Time|SetTimerbyFunctionName 0 "RevealCompleted" (Get|GetRevealDuration) false true)
    (CallFunction|NiagaraHandler (Variables|Default|GetNiagaraRevealStarted) true)))

(fn RevealCancel
  (if (== (GameplayTags|MakeLiteralGameplayTag "(TagName=\"Seal.Status.Hidden\")") (Variables|Default|GetStatus))
    (Utilities|Time|ClearTimerbyFunctionName 0 "RevealCompleted")
    (CallFunction|NiagaraHandler (Variables|Default|GetNiagaraRevealStarted) false)
    (CallFunction|NiagaraHandler (Variables|Default|GetNiagaraRevealCompleted) false)))

(fn UnsealStarted
  (if (not (Class|KismetSystemLibrary|IsTimerActive 0 "UnsealProgress"))
    (Utilities|Time|PauseTimerbyHandle (Variables|Default|GetRevealTimer))
    (Utilities|Time|SetTimerbyFunctionName 0 "UnsealProgress" (Utilities|Time|GetWorldDeltaSeconds) true)))

(fn UnsealCancel
  (if (== (GameplayTags|MakeLiteralGameplayTag "(TagName=\"Seal.Status.Revealed\")") (Variables|Default|GetStatus))
    (Utilities|Time|ClearTimerbyFunctionName 0 "UnsealProgress")
    (Utilities|Time|UnpauseTimerbyHandle (Variables|Default|GetRevealTimer))
    (Variables|Default|SetCurrentValue 0.0)))

(fn UnsealProgress
  (params (bIsAIInteraction :type Boolean))
  (if bIsAIInteraction
    (bind _output_get (Variables|Default|SetCurrentValue (+ (* (Utilities|Time|GetWorldDeltaSeconds) (Get|GetWardProgressSpeed)) (Variables|Default|GetCurrentValue))))
    (if (>= _output_get (Get|GetRequiredPoints))
      (Utilities|Time|ClearTimerbyFunctionName 0 "UnsealProgress")
      (Unseal|UnsealCompleted)
      (else
        (Development|PrintString (Utilities|String|Append "Progress: " (Utilities|String|ToString(Float) (Variables|Default|GetCurrentValue)) " / " (Utilities|String|ToString(Integer) (Get|GetRequiredPoints))) true true "(R=1.000000,G=0.738652,B=0.000000,A=1.000000)" 2.0 "ProgressUnseal")))))

(fn UnsealCompleted
  (Variables|Default|SetbIsAIInteraction false)
  (Utilities|Time|ClearandInvalidateTimerbyHandle (Variables|Default|GetRevealTimer))
  (CallFunction|AddRewardtoPlayer (Get|GetRewardValue))
  (Set|SetStatus "(TagName=\"Seal.Status.Completed\")")
  (CallFunction|RevealCancelEvent)
  (CallFunction|NiagaraHandler (Variables|Default|GetNiagaraRevealCompleted) false)
  (CallFunction|NiagaraHandler (Variables|Default|GetNiagaraUnsealCompleted) true)
  (Audio|Components|Audio|Play (Variables|Default|GetUnsealComplete) 0.0)
  (Rendering|SetVisibility (Variables|Default|GetPlane) false false))

(fn BlockedTimerExpired
  (if (== (Variables|Default|GetStatus) (GameplayTags|MakeLiteralGameplayTag "(TagName=\"Seal.Status.Blocked\")"))
    (Set|SetStatus "(TagName=\"Seal.Status.Hidden\")")
    (Variables|Default|SetCurrentValue 0.0)
    (Utilities|Time|ClearandInvalidateTimerbyHandle (Variables|Default|GetBlockedTimer))
    (Components|Activation|SetActive (Variables|Default|GetNiagaraBlocked) false false)
    (Audio|Components|Audio|Play (Variables|Default|GetSealBlockedStartEnd) 0.0)
    (Audio|Components|Audio|Stop (Variables|Default|GetSealBlockedProccesed))))

(fn BlockedStart
  (if (== (Variables|Default|GetStatus) (GameplayTags|MakeLiteralGameplayTag "(TagName=\"Seal.Status.Revealed\")"))
    (Unseal|UnsealCancel)
    (Utilities|Time|ClearandInvalidateTimerbyHandle (Variables|Default|GetRevealTimer))
    (Set|SetStatus "(TagName=\"Seal.Status.Blocked\")")
    (CallFunction|NiagaraHandler (Variables|Default|GetNiagaraRevealCompleted) false)
    (CallFunction|NiagaraHandler (Variables|Default|GetNiagaraBlocked) true)
    (Audio|Components|Audio|Play (Variables|Default|GetSealBlockedStartEnd) 0.0)
    (Audio|Components|Audio|Play (Variables|Default|GetSealBlockedProccesed) 0.0)
    (bind _returnvalue (Utilities|Time|SetTimerbyFunctionName 0 "BlockedTimerExpired" 1e+01))
    (Variables|Default|SetBlockedTimer _returnvalue)))

(fn NiagaraHandler
  (params (NiagaraEffeect :type Niagara%20Component%20Object%20Reference) (bIsActive :type Boolean))
  (if bIsActive
    (Components|Activation|SetActive NiagaraEffeect bIsActive false)
    (else
      (Components|Activation|Deactivate NiagaraEffeect))))

(fn RevealEffect
  (bind _output_get (Variables|Default|SetHoldTime (+ (Utilities|Time|GetWorldDeltaSeconds) (Variables|Default|GetHoldTime))))
  (if (Audio|Components|Audio|IsPlaying (Variables|Default|GetRevealProccesed))
    _
    (else
      (Audio|Components|Audio|Play (Variables|Default|GetSealRevealStarted) 0.0)
      (Audio|Components|Audio|Play (Variables|Default|GetRevealProccesed) 0.0)))
  (bind _output_get_2 (Variables|Default|SetRevealProgress (Math|Float|Lerp 0.0 1.0 (/ _output_get (* (Get|GetRevealDuration) 1.75)))))
  (Rendering|Material|SetCustomPrimitiveDataFloat (Variables|Default|GetPlane) 26 _output_get_2))

(fn ResetRevealEffect
  (params (Alpha :type Float%20%28double-precision%29))
  (if (Audio|Components|Audio|IsPlaying (Variables|Default|GetRevealProccesed))
    (Audio|Components|Audio|Stop (Variables|Default|GetRevealProccesed))
    (Audio|Components|Audio|Play (Variables|Default|GetSealRevealCanceled) 0.0))
  (Rendering|Material|SetCustomPrimitiveDataFloat (Variables|Default|GetPlane) 26 (Math|Float|Lerp 0.0 (Variables|Default|GetRevealProgress) Alpha)))

(fn InputActionSetting
  (params (Movement :type Boolean) (Zoom :type Boolean) (Rotate :type Boolean) (TraceInteraction :type Boolean))
  (bind _asbp_controller_base (Utilities|Casting|CastToBP_Controller_Base (Game|GetPlayerController 0)))
  (Default|InputActionSetting _asbp_controller_base Movement Zoom Rotate TraceInteraction))

(fn AIBlocked
  (if (== (GameplayTags|MakeLiteralGameplayTag "(TagName=\"Seal.Status.Revealed\")") (Variables|Default|GetStatus))
    (CallFunction|Blocked)))

(fn AIUnsealStart
  (if (== (GameplayTags|MakeLiteralGameplayTag "(TagName=\"Seal.Status.Revealed\")") (Variables|Default|GetStatus))
    (Unseal|UnsealStarted)
    (Variables|Default|SetbIsAIInteraction true)))

(fn AIUnsealCancel
  (Unseal|UnsealCancel)
  (Variables|Default|SetbIsAIInteraction false))

(fn IsFocusAvailable
  (return false))

(fn IsInteractionAvailable
  (return true))

(fn IsMainActionAvailable
  (return true))

(fn IsMainHoldActionAvailable
  (return true))

(fn IsSecondActionAvailable
  (return true))

(fn IsSecondHoldActionAvailable
  (return false))
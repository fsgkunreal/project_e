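; Ward character Blueprint that tracks temporary and permanent stress through a ModifierManager, which is seeded at BeginPlay and ticks effects.
; AddStress adds modifiers scaled by source-specific coefficient tags, then UpdateStressStage compares their sum against thresholds.
; Stage changes swap state flags and data-asset effects and fire OnStressStateChanged, except entering Calm, which only clears the old stage.
; Disconnected debug chains exercise stress, modifiers and effects.
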(event EventBeginPlay
  ;[0.1301 0.1274 0.1301 1 14] Установить базовые значения стресса, коэффициентов, скорости накопления очков распечатывания и порогов в ModifierManagerComponent
  (|CallParentFunction)
  (Default|SetBaseValues (Variables|Default|GetModifierManager) (Variables|Default|GetBaseValues))
  (CallFunction|AddFlag "(TagName=\"State.Stress.Calm\")"))

(event EventTick
  (params (DeltaSeconds :type Float%20%28single-precision%29))
  (|CallParentFunction DeltaSeconds)
  (Utilities|FlowControl|Sequence
    (:then_1
      (Default|TickEffects (Variables|Default|GetModifierManager) DeltaSeconds))))

(fn ConstructionScript)

(fn AddStress
  (params (SourceType :type StressSourceType%20Enum :default "NewEnumerator0") (Value :type Float%20%28double-precision%29))
  (Default|AddModifier (Variables|Default|GetModifierManager) (Utilities|Struct|MakeF_Modifier (GameplayTags|MakeLiteralGameplayTag "(TagName=\"Stat.Stress.Temporary\")") "NewEnumerator0" Value true true (GameplayTags|MakeGameplayTagContainerfromArray (Utilities|Array|MakeArray (GameplayTags|MakeLiteralGameplayTag "(TagName=\"Stat.Stress.Coefficient.Temporary\")") (StressCore|GetCoefficientTag SourceType)))))
  (Default|AddModifier (Variables|Default|GetModifierManager) (Utilities|Struct|MakeF_Modifier (GameplayTags|MakeLiteralGameplayTag "(TagName=\"Stat.Stress.Permanent\")") "NewEnumerator0" Value true true (GameplayTags|MakeGameplayTagContainerfromArray (Utilities|Array|MakeArray (GameplayTags|MakeLiteralGameplayTag "(TagName=\"Stat.Stress.Coefficient.Permanent\")") (GameplayTags|MakeLiteralGameplayTag "(TagName=\"Stat.Stress.Coefficient.Temporary\")") (StressCore|GetCoefficientTag SourceType)))))
  (StateManagement|UpdateStressStage))

(fn GetCoefficientTag
  (params (SourceType :type StressSourceType%20Enum :default "NewEnumerator0"))
  (switch Utilities|FlowControl|Switch|SwitchonStressSourceType SourceType
    (:NewEnumerator0
      (return "(TagName=\"Stat.Stress.Coefficient.Darkness\")"))
    (:NewEnumerator1
      (return "(TagName=\"Stat.Stress.Coefficient.Noise\")"))
    (:NewEnumerator2
      (return "(TagName=\"Stat.Stress.Coefficient.Supernatural\")"))
    (:NewEnumerator3
      (return "(TagName=\"Stat.Stress.Coefficient.Aggressive\")"))
    (:NewEnumerator4
      (return "(TagName=\"Stat.Stress.Coefficient.EnemyNotice\")"))
    (:NewEnumerator5
      (return "(TagName=\"Stat.Stress.Coefficient.ChaseBegin\")"))
    (:NewEnumerator6
      (return "(TagName=\"Stat.Stress.Coefficient.Trap\")"))))

(fn GetTargetStressState
  (bind _modifiermanager (Variables|Default|GetModifierManager))
  (bind _value (Default|GetFinalValue _modifiermanager "(TagName=\"Stat.Stress.Permanent\")"))
  (bind _value_2 (Default|GetFinalValue _modifiermanager "(TagName=\"Stat.Stress.Temporary\")"))
  (bind _returnvalue (+ _value_2 _value))
  (if (>= _returnvalue (Default|GetFinalValue _modifiermanager "(TagName=\"Stat.Stress.Threshold.Panic\")"))
    (return "(TagName=\"State.Stress.Panic\")")
    (elif (>= _returnvalue (Default|GetFinalValue _modifiermanager "(TagName=\"Stat.Stress.Threshold.Mobilization\")"))
      (return "(TagName=\"State.Stress.OnTheEdge\")")
      (elif (>= _returnvalue (Default|GetFinalValue _modifiermanager "(TagName=\"Stat.Stress.Threshold.Calm\")"))
        (return "(TagName=\"State.Stress.Mobilization\")")
        (else
          (return "(TagName=\"State.Stress.Calm\")"))))))

(fn GetCurrentStressState
  (if (CallFunction|HasFlag "(TagName=\"State.Stress.Panic\")")
    (return "(TagName=\"State.Stress.Panic\")")
    (elif (CallFunction|HasFlag "(TagName=\"State.Stress.OnTheEdge\")")
      (return "(TagName=\"State.Stress.OnTheEdge\")")
      (elif (CallFunction|HasFlag "(TagName=\"State.Stress.Mobilization\")")
        (return "(TagName=\"State.Stress.Mobilization\")")
        (else
          (return "(TagName=\"State.Stress.Calm\")"))))))

(fn UpdateStressStage
  (bind _currentstate (StateDetection|GetCurrentStressState))
  (bind _targetstate (StateDetection|GetTargetStressState))
  (bind _effect (Utility|GetEffectHandleforState _targetstate))
  (bind _effectdata (Utilities|Struct|BreakF_StatusEffectHandle _effect))
  (if (not (== _targetstate _currentstate))
    (CallFunction|RemoveFlag _currentstate)
    (Default|RemoveEffect (Variables|Default|GetModifierManager) (Utility|GetEffectHandleforState _currentstate))
    (if (!= _targetstate "(TagName=\"State.Stress.Calm\")")
      (CallFunction|AddFlag _targetstate)
      (Default|ApplyEffect (Variables|Default|GetModifierManager) _effectdata _effectdata)
      (Default|CallOnStressStateChanged _targetstate))))

(fn GetEffectHandleforState
  (params (State :type Gameplay%20Tag%20Structure))
  (if (== State (GameplayTags|MakeLiteralGameplayTag "(TagName=\"State.Stress.Panic\")"))
    (return (LocalVariables|GetDA_Panic))
    (elif (== State (GameplayTags|MakeLiteralGameplayTag "(TagName=\"State.Stress.OnTheEdge\")"))
      (return (LocalVariables|GetDA_OnTheEdge))
      (elif (== State (GameplayTags|MakeLiteralGameplayTag "(TagName=\"State.Stress.Mobilization\")"))
        (return (LocalVariables|GetDA_Mobilization))
        (else
          (return (LocalVariables|GetDA_Calm)))))))
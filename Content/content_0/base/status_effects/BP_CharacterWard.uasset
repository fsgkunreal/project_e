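; BP_CharacterWard is a ward character Blueprint that tracks stress and sorts it into gameplay-tag stages.
; AddStress scales incoming stress by a ModifierManager value for its source, accumulates it as temporary stress, then refreshes the stage.
; UpdateStressStage tests temporary plus permanent stress against ModifierManager thresholds for Panic, Mobilization and Calm, falling back to OnTheEdge below Calm.
; On a change it swaps the State.Stress flag and broadcasts OnStressStateChanged.
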(event EventBeginPlay
  (|CallParentFunction) ; This node is disabled and will not be called.\nDrag off pins to build functionality.
)

(event Collision|EventActorBeginOverlap
  (params (OtherActor :type Actor%20Object%20Reference))
  (|CallParentFunction OtherActor) ; This node is disabled and will not be called.\nDrag off pins to build functionality.
)

(event EventTick
  (params (DeltaSeconds :type Float%20%28single-precision%29))
  (|CallParentFunction DeltaSeconds) ; This node is disabled and will not be called.\nDrag off pins to build functionality.
)

(fn ConstructionScript
  (|CallParentFunction))

(fn AddStress
  (params (Value :type Float%20%28double-precision%29) (SourceType :type Gameplay%20Tag%20Structure))
  (Variables|Default|SetStressTemporary (+ (* Value (Default|GetFinalValue (Variables|Default|GetModifierManager) SourceType)) (Variables|Default|GetStressTemporary)))
  (CallFunction|UpdateStressStage))

(fn UpdateStressStage
  (bind _stresstemporary (Variables|Default|GetStressTemporary))
  (bind _stresspermanent (Variables|Default|GetStressPermanent))
  (bind _modifiermanager (Variables|Default|GetModifierManager))
  (bind _returnvalue (+ _stresstemporary _stresspermanent))
  (Utilities|FlowControl|Sequence
    (:then_0
      (LocalVariables|SetCurrentState "")
      (bind _array_element (Utilities|Array|ForEachLoopwithBreak (GameplayTags|BreakGameplayTagContainer (CallFunction|GetFlags)) :!label _label)
        (:LoopBody
          (if (GameplayTags|MatchesTag _array_element "(TagName=\"State.Stress\")")
            (LocalVariables|SetCurrentState _array_element)
            (goto _label Break)))))
    (:then_1
      (if (>= _returnvalue (Default|GetFinalValue _modifiermanager "(TagName=\"State.Stress.Panic\")"))
        (LocalVariables|SetNewState "(TagName=\"State.Stress.Panic\")")
        (elif (>= _returnvalue (Default|GetFinalValue _modifiermanager "(TagName=\"State.Stress.Mobilization\")"))
          (LocalVariables|SetNewState "(TagName=\"State.Stress.Mobilization\")")
          (elif (>= _returnvalue (Default|GetFinalValue _modifiermanager "(TagName=\"State.Stress.Calm\")"))
            (LocalVariables|SetNewState "(TagName=\"State.Stress.Calm\")")
            (else
              (LocalVariables|SetNewState "(TagName=\"State.Stress.OnTheEdge\")"))))))
    (:then_2
      (if (!= (LocalVariables|GetNewState) (LocalVariables|GetCurrentState))
        (CallFunction|RemoveFlag (LocalVariables|GetCurrentState))
        (CallFunction|AddFlag (LocalVariables|GetNewState))
        (Default|CallOnStressStateChanged (LocalVariables|GetNewState))))))
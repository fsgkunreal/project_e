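; Test actor that exercises a ModifierManagerComponent for status effects and stat modifiers, reporting results through on-screen prints.
; Tick advances the component's effects, and BeginPlay prints the final MoveSpeed value.
; Disconnected graph chains hold manual scenarios for effect priority, reapplying a speed effect, and comparing base against final values.
; Helper functions wrap setting, reading, modifier and effect calls, but the live events call none of them.
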(event EventBeginPlay
  (Utilities|FlowControl|Sequence
    (:then_0
      (Development|PrintString (Utilities|String|ToString(Float) (Default|GetFinalValue (Variables|Default|GetModifierManagerComponent) "(TagName=\"Stat.MoveSpeed\")")) true true "(R=0.000000,G=0.660000,B=1.000000,A=1.000000)" 5e+01))))

(event EventTick
  (params (DeltaSeconds :type Float%20%28single-precision%29))
  (Default|TickEffects (Variables|Default|GetModifierManagerComponent) DeltaSeconds))

(fn ConstructionScript)

(fn PrintFinalValue
  (Development|PrintString "GetFinalValue" true true "(R=0.000000,G=0.660000,B=1.000000,A=1.000000)" 1e+02)
  (Development|PrintString (Utilities|String|ToString(Float) (Default|GetFinalValue (Variables|Default|GetModifierManagerComponent) "(TagName=\"Stat.MoveSpeed\")")) true true "(R=0.000000,G=0.660000,B=1.000000,A=1.000000)" 1e+02))

(fn SetBaseValue
  (bind _testtag (Variables|Default|GetTestTag))
  (bind _testvalue (Variables|Default|GetTestValue))
  (Default|SetBaseValue (Variables|Default|GetModifierManagerComponent) _testtag _testvalue)
  (Development|PrintString "BaseValueSet" true true "(R=0.000000,G=0.660000,B=1.000000,A=1.000000)" 1e+01)
  (Development|PrintString (GameplayTags|GetDebugStringfromGameplayTag _testtag) true true "(R=0.000000,G=0.660000,B=1.000000,A=1.000000)" 1e+01)
  (Development|PrintString (Utilities|String|ToString(Float) _testvalue) true true "(R=0.000000,G=0.660000,B=1.000000,A=1.000000)" 1e+01))

(fn TestGetBaseValue
  (Development|PrintString "GetBaseValue" true true "(R=1.000000,G=0.019054,B=0.000000,A=1.000000)" 5.0)
  (Development|PrintString (Utilities|String|ToString(Float) (Default|GetBaseValue (Variables|Default|GetModifierManagerComponent) (Variables|Default|GetTestTag))) true true "(R=1.000000,G=0.019054,B=0.000000,A=1.000000)" 5.0))

(fn TestGetFinalValue
  (Development|PrintString "GetFinalValue" true true "(R=1.000000,G=0.968910,B=0.000000,A=1.000000)" 5.0)
  (Development|PrintString (Utilities|String|ToString(Float) (Default|GetFinalValue (Variables|Default|GetModifierManagerComponent) (Variables|Default|GetTestTag))) true true "(R=1.000000,G=0.968910,B=0.000000,A=1.000000)" 5.0))

(fn TestAddDirectModifier)

(fn TestAddMultiplyModifier
  (Default|AddModifier (Variables|Default|GetModifierManagerComponent) (Utilities|Struct|MakeF_Modifier (Variables|Default|GetTestTag) "NewEnumerator1" 0.8))
  (Development|PrintString "Added multiply modifier" true true "(R=0.003198,G=1.000000,B=0.159362,A=1.000000)" 5.0)
  (Development|PrintString "0.8" true true "(R=0.003198,G=1.000000,B=0.159362,A=1.000000)" 5.0))

(fn AddApplyEffect
  (bind _effect (Variables|Default|GetEffect))
  (Default|ApplyEffect (Variables|Default|GetModifierManagerComponent) _effect _effect)
  (Development|PrintString "ApplyEffects" true true "(R=0.000000,G=0.660000,B=1.000000,A=1.000000)" 1e+02)
  (Development|PrintString "____________________" true true "(R=0.000000,G=0.660000,B=1.000000,A=1.000000)" 1e+02)
  (CallFunction|PrintFinalValue))
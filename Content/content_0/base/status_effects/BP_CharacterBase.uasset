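; Base character Blueprint for the status effects content, exposing a modifier manager and a set of gameplay-tag flags.
; Accessor functions return the ModifierManager and the Flags container, while HasFlag, AddFlag and RemoveFlag query or edit the container's tags directly.
; It adds no event or construction logic of its own.
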(event EventBeginPlay)

(event Collision|EventActorBeginOverlap
  (params (OtherActor :type Actor%20Object%20Reference)))

(event EventTick
  (params (DeltaSeconds :type Float%20%28single-precision%29)))

(fn ConstructionScript)

(fn GetModifierManager
  (return (Variables|Default|GetModifierManager)))

(fn HasFlag
  (params (Flag :type Gameplay%20Tag%20Structure))
  (return (Utilities|Array|ContainsItem (GameplayTags|BreakGameplayTagContainer (Variables|Default|GetFlags)) Flag)))

(fn AddFlag
  (params (Flag :type Gameplay%20Tag%20Structure))
  (Utilities|Array|Add (GameplayTags|BreakGameplayTagContainer (Variables|Default|GetFlags)) Flag))

(fn RemoveFlag
  (params (Flag :type Gameplay%20Tag%20Structure))
  (Utilities|Array|RemoveItem (GameplayTags|BreakGameplayTagContainer (Variables|Default|GetFlags)) Flag))

(fn GetFlags
  (return (Variables|Default|GetFlags)))
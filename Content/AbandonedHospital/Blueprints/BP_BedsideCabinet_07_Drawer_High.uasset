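; Bedside cabinet prop with a drawer for the Abandoned Hospital level, wired for hover feedback only.
; Hover start applies an overlay material to the Drawer component and hover end clears it, each printing a debug string to screen.
; All availability checks for focus mode, interaction, and main, second and hold actions return false, so the drawer offers no actions.
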(event EventOnHoverStart
  (Rendering|Material|SetOverlayMaterial (Variables|Default|GetDrawer) "/Game/content_0/interfaces/M_Overlay.M_Overlay" :!class /Script/Engine.MeshComponent)
  (Development|PrintString "OnHoverStart" true true "(R=1.000000,G=0.968910,B=0.000000,A=1.000000)" 2.0 "3"))

(event EventOnHoverEnd
  (Rendering|Material|SetOverlayMaterial (Variables|Default|GetDrawer) 0 :!class /Script/Engine.MeshComponent)
  (Development|PrintString "OnHoverEnd" true true "(R=1.000000,G=0.968910,B=0.000000,A=1.000000)" 2.0 "3"))

(fn ConstructionScript)

(fn IsFocusModeAvailable
  (return false))

(fn IsInteractionAvailable
  (return false))

(fn IsMainActionAvailable
  (return false))

(fn IsMainHoldActionAvailable
  (return false))

(fn IsSecondActionAvailable
  (return false))

(fn IsSecondHoldActionAvailable
  (return false))
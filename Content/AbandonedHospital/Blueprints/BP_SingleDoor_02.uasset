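; Interactive single door actor that the player opens and closes with the Interact input while inside its proximity trigger, unless it is locked.
; The trigger sets readiness and fades two world-space widget prompts in and out, showing either "Press E" or "Locked".
; A FlipFlop alternates open and close animations on the skeletal mesh, with cross-reset DoOnce gates and delays blocking each action until the previous animation finishes.
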(event OnComponentBeginOverlap(Proxy_B)
  (params (OverlappedComponent :type Primitive%20Component%20Object%20Reference) (OtherActor :type Actor%20Object%20Reference) (OtherComp :type Primitive%20Component%20Object%20Reference) (OtherBodyIndex :type Integer) (bFromSweep :type Boolean) (SweepResult :type Hit%20Result%20Structure%20%28by%20ref%29))
  (Variables|Default|SetReady_To_Open? true)
  (if (Variables|Default|GetLocked?)
    (Default|PlayFadein (Variables|Default|GetWB_Locked_01))
    (Rendering|SetVisibility (Variables|Default|GetLocked_A) true false)
    (else
      (Default|PlayFadein (Variables|Default|GetWB_PressE_01))
      (Rendering|SetVisibility (Variables|Default|GetPressE_A) true false))))

(event OnComponentEndOverlap(Proxy_B)
  (params (OverlappedComponent :type Primitive%20Component%20Object%20Reference) (OtherActor :type Actor%20Object%20Reference) (OtherComp :type Primitive%20Component%20Object%20Reference) (OtherBodyIndex :type Integer))
  (Variables|Default|SetReady_To_Open? false)
  (if (Variables|Default|GetLocked?)
    (Default|PlayFadeOut (Variables|Default|GetWB_Locked_01))
    (Utilities|FlowControl|Delay 1.0)
    (Rendering|SetVisibility (Variables|Default|GetLocked_A) false false)
    (else
      (Default|PlayFadeOut (Variables|Default|GetWB_PressE_01))
      (Utilities|FlowControl|Delay 1.0)
      (Rendering|SetVisibility (Variables|Default|GetPressE_A) false false))))

(event EventBeginPlay
  (Utilities|Casting|CastToBP_FirstPersonCharacter (Game|GetPlayerCharacter 0))
  (Input|EnableInput (Game|GetPlayerController 0))
  (bind _aswb_press_e (Utilities|Casting|CastToWB_PressE (UserInterface|GetUserWidgetObject (Variables|Default|GetPressE_A))))
  (Variables|Default|SetWB_PressE_01 _aswb_press_e)
  (bind _aswb_press_e_2 (Utilities|Casting|CastToWB_PressE (UserInterface|GetUserWidgetObject (Variables|Default|GetPressE_B))))
  (Variables|Default|SetWB_PressE_02 _aswb_press_e_2)
  (bind _aswb_locked (Utilities|Casting|CastToWB_Locked (UserInterface|GetUserWidgetObject (Variables|Default|GetLocked_A))))
  (Variables|Default|SetWB_Locked_01 _aswb_locked)
  (bind _aswb_locked_2 (Utilities|Casting|CastToWB_Locked (UserInterface|GetUserWidgetObject (Variables|Default|GetLocked_B))))
  (Variables|Default|SetWB_Locked_02 _aswb_locked_2))

(event Collision|EventActorBeginOverlap
  (params (OtherActor :type Actor%20Object%20Reference)))

(event EventTick
  (params (DeltaSeconds :type Float%20%28single-precision%29)))

(event Input|ActionEvents|InputActionInteract
  (params (Key :type Key%20Structure))
  (:Pressed
    (if (not (Variables|Default|GetLocked?))
      (if (Variables|Default|GetReady_To_Open?)
        (Utilities|FlowControl|FlipFlop
          (:A
            (Utilities|FlowControl|DoOnce false :!label _label
              (:Completed
                (Components|Animation|PlayAnimation (Variables|Default|GetSM_DoorSingle_02) "/Game/AbandonedHospital/Animations/AS_DoorSingle_02_Open.AS_DoorSingle_02_Open" false)
                (Utilities|FlowControl|Delay 1.8)
                (goto _label_2 Reset))))
          (:B
            (Utilities|FlowControl|DoOnce true :!label _label_2
              (:Completed
                (Components|Animation|PlayAnimation (Variables|Default|GetSM_DoorSingle_02) "/Game/AbandonedHospital/Animations/AS_DoorSingle_02_Close.AS_DoorSingle_02_Close" false)
                (Utilities|FlowControl|Delay 1.8)
                (goto _label Reset)))))))))

(fn ConstructionScript)
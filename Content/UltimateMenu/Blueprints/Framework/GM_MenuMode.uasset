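; GM_MenuMode is the game mode for the UltimateMenu framework.
; On PostLogin it appends each joining controller to a Player array, and GetPlayerOnSession returns that array's length as text.
; FindMainPlayerStart searches all PlayerStart actors and returns the first whose tag matches MainPlayerStartTag.
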(event EventPostLogin
  (params (NewPlayer :type Player%20Controller%20Object%20Reference))
  (Utilities|Array|Add (Variables|Default|GetPlayer) NewPlayer))

(fn ConstructionScript)

(fn FindMainPlayerStart
  (bind _outactors (Actor|GetAllActorsOfClass "/Script/Engine.PlayerStart"))
  (bind _array_element (Utilities|Array|ForEachLoopwithBreak _outactors :!label _label)
    (:LoopBody
      (if (Utilities|Name|Equal(Name) (Variables|/Script/Engine.PlayerStart|GetPlayerStartTag _array_element) (Variables|Default|GetMainPlayerStartTag))
        (LocalVariables|SetLocReturn _array_element)
        (goto _label Break)))
    (:Completed
      (return (LocalVariables|GetLocReturn)))))

(fn GetPlayeronSession
  (return (Utilities|Text|ToText(Integer) (Utilities|Array|Length (Variables|Default|GetPlayer)))))
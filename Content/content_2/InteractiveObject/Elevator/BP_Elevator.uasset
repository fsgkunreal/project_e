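; BP_Elevator is an interactive elevator whose two doors slide open when the player performs the main action.
; The action plays a door-open sound and runs a timeline that lerps the right and left door meshes apart along their relative Y axis.
; Hovering toggles an outline overlay material on the board mesh, and availability functions allow only interaction and the main action, with no focus, hold or secondary actions.
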(event EventDoMainAction
  (params (HitResult :type Hit%20Result%20Structure))
  (Audio|PlaySound2D "/Game/content_2/Doors_And_Drawers_SFX/Elevator/Elevator_Door_Open/WAV_Elevator_Door_Open_1.WAV_Elevator_Door_Open_1" 1.0 1.0 0.0 0 0)
  (bind _alpha (Timeline|Timeline Play)
    (:Update
      (Transformation|SetRelativeLocation (Variables|Default|GetSM_Elevator_Door_Right) (Math|Vector|MakeVector 0.0 (Math|Float|Lerp 0.0 -8e+01 _alpha) 0.0) false false)
      (Transformation|SetRelativeLocation (Variables|Default|GetSM_Elevator_Door_Left) (Math|Vector|MakeVector 0.0 (Math|Float|Lerp 0.0 8e+01 _alpha) 0.0) false false))))

(event EventOnHoverStart
  (Rendering|Material|SetOverlayMaterial (Variables|Default|GetSM_ElevatorBoard) "/Game/content_2/InteractiveObject/Effects/MI_Outline.MI_Outline" :!class /Script/Engine.MeshComponent))

(event EventOnHoverEnd
  (Rendering|Material|SetOverlayMaterial (Variables|Default|GetSM_ElevatorBoard) 0 :!class /Script/Engine.MeshComponent))

(fn ConstructionScript)

(fn IsFocusAvailable
  (return false))

(fn IsInteractionAvailable
  (return true))

(fn IsMainActionAvailable
  (return true))

(fn IsMainHoldActionAvailable
  (return false))

(fn IsSecondActionAvailable
  (return false))

(fn IsSecondHoldActionAvailable
  (return false))
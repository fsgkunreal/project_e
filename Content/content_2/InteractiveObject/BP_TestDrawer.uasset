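; Focusable drawer cabinet that gathers its child BP_Drawer actors and spawns an item in a random one, simulating its physics only during focus.
; On keyboard layouts, focus enables interaction on every drawer.
; On gamepad, main and secondary actions step through drawers with an orange overlay highlight.
; Holding main projects camera-relative input onto the cabinet's forward axis and passes it to the selected drawer.
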(event EventBeginPlay
  (bind _drawerarray (Variables|Default|GetDrawerArray))
  (bind _arrayelement (Utilities|Array|ReverseforEachLoop (Actor|GetAllChildActors true))
    (:LoopBody
      (bind _asbp_drawer (Utilities|Casting|CastToBP_Drawer _arrayelement))
      (Utilities|Array|Add (Variables|Default|GetDrawerArray) _asbp_drawer))
    (:Completed
      (Variables|Default|SetDrawerOnHover (Utilities|Array|Get(acopy) _drawerarray (Variables|Default|GetDrawerIndex)))
      (bind _item (Default|SpawnItem (.OutItem (Utilities|Array|Random _drawerarray))))
      (Variables|Default|SetInnerItem _item))))

(event EventOnFocusStart
  (bind _body (Variables|Default|GetBody))
  (bind _output_get (Variables|Default|SetbIsOnFocus true))
  (Physics|SetSimulatePhysics (Variables|/Game/content_0/base/throwable/BP_Throwable.BP_Throwable_C|GetMesh (Variables|Default|GetInnerItem)) _output_get)
  (bind _bisgamepad (CallFunction|GetControllerLayout))
  (if _bisgamepad
    (Rendering|Material|SetOverlayMaterial (Variables|/Game/content_0/base/drawer/BP_Drawer.BP_Drawer_C|GetStaticMesh (Variables|Default|GetDrawerOnHover)) "/Game/content_0/interfaces/M_Overlay_Orange.M_Overlay_Orange" :!class /Script/Engine.MeshComponent)
    (Rendering|Material|SetOverlayMaterial _body 0 :!class /Script/Engine.MeshComponent)
    (else
      (CallFunction|DrawerInteractionHandler true)
      (Rendering|Material|SetOverlayMaterial _body 0 :!class /Script/Engine.MeshComponent))))

(event EventOnFocusEnd
  (bind _output_get (Variables|Default|SetbIsOnFocus false))
  (Physics|SetSimulatePhysics (Variables|/Game/content_0/base/throwable/BP_Throwable.BP_Throwable_C|GetMesh (Variables|Default|GetInnerItem)) _output_get)
  (Utilities|FlowControl|Sequence
    (:then_0
      (Rendering|Material|SetOverlayMaterial (Variables|/Game/content_0/base/drawer/BP_Drawer.BP_Drawer_C|GetStaticMesh (Variables|Default|GetDrawerOnHover)) 0 :!class /Script/Engine.MeshComponent))
    (:then_1
      (CallFunction|DrawerInteractionHandler false))))

(event EventTick
  (params (DeltaSeconds :type Float%20%28single-precision%29))
  (bind _drawerindex (Variables|Default|GetDrawerIndex))
  (bind _drawerarray (Variables|Default|GetDrawerArray))
  (bind _output (Utilities|Array|Get(acopy) _drawerarray _drawerindex))
  (bind _bisgamepad (CallFunction|GetControllerLayout))
  (if _bisgamepad
    (if (!= _output (Variables|Default|GetDrawerOnHover))
      (Rendering|Material|SetOverlayMaterial (Variables|/Game/content_0/base/drawer/BP_Drawer.BP_Drawer_C|GetStaticMesh (Variables|Default|GetDrawerOnHover)) 0 :!class /Script/Engine.MeshComponent)
      (bind _output_get (Variables|Default|SetDrawerOnHover _output))
      (Rendering|Material|SetOverlayMaterial (Variables|/Game/content_0/base/drawer/BP_Drawer.BP_Drawer_C|GetStaticMesh _output_get) "/Game/content_0/interfaces/M_Overlay_Orange.M_Overlay_Orange" :!class /Script/Engine.MeshComponent))))

(event EventOnHoverStart
  (if (Variables|Default|GetbIsOnFocus)
    (Rendering|Material|SetOverlayMaterial (Variables|Default|GetBody) 0 :!class /Script/Engine.MeshComponent)
    (else
      (Rendering|Material|SetOverlayMaterial (Variables|Default|GetBody) "/Game/content_0/interfaces/M_Overlay_Orange.M_Overlay_Orange" :!class /Script/Engine.MeshComponent))))

(event EventOnHoverEnd
  (if (not (Variables|Default|GetbIsOnFocus))
    (Rendering|Material|SetOverlayMaterial (Variables|Default|GetBody) 0 :!class /Script/Engine.MeshComponent)))

(event EventDoMainAction
  (params (HitResult :type Hit%20Result%20Structure))
  (if (<= (+ 1 (Variables|Default|GetDrawerIndex)) (- (Utilities|Array|Length (Variables|Default|GetDrawerArray)) 1))
    (Variables|Default|SetDrawerIndex (+ 1 (Variables|Default|GetDrawerIndex)))))

(event EventDoSecondAction
  (if (>= (- (Variables|Default|GetDrawerIndex) 1) 0)
    (Variables|Default|SetDrawerIndex (- (Variables|Default|GetDrawerIndex) 1))))

(event EventDoMainActionHold
  (params (HoldTime :type Float%20%28double-precision%29) (Direction :type Vector%202D%20Structure))
  (CallFunction|GamepadDrawerInteraction Direction))

(fn ConstructionScript)

(fn GamepadDrawerInteraction
  (params (Direction :type Vector%202D%20Structure))
  (bind _returnvalue (Game|GetPlayerCameraManager 0))
  (bind _result (Math|Float|NegateFloat (Math|Vector|DotProduct (Math|Vector|Normalize (+ (* (.x Direction) (Transformation|GetActorRightVector _returnvalue)) (Math|Vector|NegateVector (* (Transformation|GetActorForwardVector _returnvalue) (.y Direction))))) (Transformation|GetActorForwardVector)))
    (:%20%20
      (Default|GamepadDrawerInteraction (Variables|Default|GetDrawerOnHover) _result))))

(fn DrawerInteractionHandler
  (params (bIsInteractionAvailable :type Boolean))
  (for _array_element (Variables|Default|GetDrawerArray)
    (Default|InteractionHandler _array_element bIsInteractionAvailable)))

(fn GetControllerLayout
  (bind _asmy_game_instance (Utilities|Casting|CastToMyGameInstance (Game|GetGameInstance)))
  (switch Utilities|FlowControl|Switch|SwitchonE_ControlLayout (Default|GetControlLayout _asmy_game_instance)
    (:NewEnumerator0
      _)
    (:NewEnumerator1
      _)
    (:NewEnumerator2
      (return true)))
  (return false))

(fn IsFocusAvailable
  (return true))

(fn IsInteractionAvailable
  (return true))

(fn IsMainActionAvailable
  (return true))

(fn IsMainHoldActionAvailable
  (return true))

(fn IsSecondActionAvailable
  (return true))

(fn IsSecondHoldActionAvailable
  (return false))
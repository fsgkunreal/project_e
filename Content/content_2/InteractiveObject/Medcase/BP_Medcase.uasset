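; BP_Medcase is an interactive medical case whose lid opens and closes on the main action.
; Each action picks the open or closed roll from IsClosed, flips that state through a FlipFlop and replays a Timeline that lerps Upper from its current roll toward the target.
; Hover applies an outline overlay material to Upper and Lower.
; Availability functions allow interaction and main action only, disabling focus, hold and secondary actions.
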(event EventDoMainAction
  (params (HitResult :type Hit%20Result%20Structure))
  (if (Variables|Default|GetbIsClosed)
    (Variables|Default|SetTemporaryB (Variables|Default|GetOpenX))
    (else
      (Variables|Default|SetTemporaryB (Variables|Default|GetClosedX))))
  (Utilities|FlowControl|FlipFlop
    (:A
      (Variables|Default|SetbIsClosed false)
      (bind _alpha (Timeline|Timeline PlayFromStart)
        (:Update
          (Transformation|SetRelativeRotation (Variables|Default|GetUpper) (Math|Rotator|MakeRotator (Math|Float|Lerp (.roll (Variables|/Script/Engine.SceneComponent|GetRelativeRotation (Variables|Default|GetUpper))) (Variables|Default|GetTemporaryB) _alpha) 0.0 0.0) false false))))
    (:B
      (Variables|Default|SetbIsClosed true)
      (Timeline|Timeline PlayFromStart))))

(event EventOnHoverStart
  (params (CurrentControlLayout :type E_ControlLayout%20Enum :default "NewEnumerator0"))
  (Rendering|Material|SetOverlayMaterial (Variables|Default|GetUpper) "/Game/content_2/InteractiveObject/Effects/MI_Outline.MI_Outline" :!class /Script/Engine.MeshComponent)
  (Rendering|Material|SetOverlayMaterial (Variables|Default|GetLower) "/Game/content_2/InteractiveObject/Effects/MI_Outline.MI_Outline" :!class /Script/Engine.MeshComponent))

(event EventOnHoverEnd
  (params (CurrentControlLayout :type E_ControlLayout%20Enum :default "NewEnumerator0"))
  (Rendering|Material|SetOverlayMaterial (Variables|Default|GetUpper) 0 :!class /Script/Engine.MeshComponent)
  (Rendering|Material|SetOverlayMaterial (Variables|Default|GetLower) 0 :!class /Script/Engine.MeshComponent))

(fn ConstructionScript)

(fn IsFocusAvailable
  (return false))

(fn IsInteractionAvailable
  (return true))

(fn IsMainActionAvailable
  (return true))

(fn IsMainHoldActionAvailable
  (return false))

(fn IsSecondActionAvailable
  (return false))

(fn IsSecondHoldActionAvailable
  (return false))
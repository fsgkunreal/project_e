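; Interactable storage prop that the player can topple once, triggering a reaction from a nearby doctor enemy.
; The main action enables physics on all its static meshes, disables further interaction and launches the body with a fixed world-space impulse.
; A timer freezes physics five seconds later, while a sphere overlap calls HCFireExstReaction on the first doctor found.
; Hovering toggles an outline overlay while interaction is available.
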(event EventOnHoverStart
  (params (CurrentControlLayout :type E_ControlLayout%20Enum :default "NewEnumerator0"))
  (if (Variables|Default|GetInteractiveAvailable)
    (Rendering|Material|SetOverlayMaterial (Variables|Default|GetSM_Body) "/Game/content_2/InteractiveObject/Effects/MI_Outline.MI_Outline" :!class /Script/Engine.MeshComponent)))

(event EventOnHoverEnd
  (params (CurrentControlLayout :type E_ControlLayout%20Enum :default "NewEnumerator0"))
  (Rendering|Material|SetOverlayMaterial (Variables|Default|GetSM_Body) 0 :!class /Script/Engine.MeshComponent))

(event EventDoMainAction
  (params (HitResult :type Hit%20Result%20Structure))
  (CallFunction|EnablePhysyc)
  (Physics|AddImpulse (Variables|Default|GetSM_Body) "-800.000000,0.000000,0.000000" "None" true)
  (Utilities|Time|SetTimerbyFunctionName 0 "DisablePhysyc" 5.0)
  (bind _outactors (Collision|SphereOverlapActors (Transformation|GetActorLocation) 3e+02 (Utilities|Array|MakeArray "ObjectTypeQuery1" "ObjectTypeQuery3") "/Game/content_1/scripts/ai/characters/humans/character_enemy_doctor.character_enemy_doctor_C"))
  (bind _ascharacter_enemy_doctor (Utilities|Casting|CastTocharacter_enemy_doctor (Utilities|Array|Get(acopy) _outactors)))
  (Default|HCFireExstReaction _ascharacter_enemy_doctor))

(event EventBeginPlay
  (for _array_element (Actor|GetComponentsByClass "/Script/Engine.StaticMeshComponent")
    (if (!= (Variables|Default|GetSM_Body) _array_element)
      (Utilities|Array|Add (Variables|Default|GetArray) _array_element)))
  (Physics|SetSimulatePhysics (Variables|Default|GetSM_Body) false))

(fn ConstructionScript)

(fn EnablePhysyc
  (for _array_element (Variables|Default|GetArray)
    (Physics|SetSimulatePhysics _array_element true))
  (Physics|SetSimulatePhysics (Variables|Default|GetSM_Body) true)
  (Variables|Default|SetInteractiveAvailable false)
  (return true))

(fn DisablePhysyc
  (for _array_element (Variables|Default|GetArray)
    (Physics|SetSimulatePhysics _array_element false))
  (Physics|SetSimulatePhysics (Variables|Default|GetSM_Body) false)
  (Development|PrintString "Physycs Disable" true true "(R=0.000000,G=0.660000,B=1.000000,A=1.000000)" 25.0))

(fn IsFocusAvailable
  (return false))

(fn IsInteractionAvailable
  (return (Variables|Default|GetInteractiveAvailable)))

(fn IsMainActionAvailable
  (return true))

(fn IsMainHoldActionAvailable
  (return false))

(fn IsSecondActionAvailable
  (return false))

(fn IsSecondHoldActionAvailable
  (return false))
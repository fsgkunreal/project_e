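; Interactive fuse box that the player can trigger once to blow it and get the reaction of a nearby enemy doctor.
; Hover outlines body and door via overlay material while interaction remains available.
; The main action disables interaction, clears the outline, briefly fires two spark effects and launches the door with physics and a random impulse.
; A sphere overlap then passes the box's location to the first doctor found.
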(event EventOnHoverStart
  (if (Variables|Default|GetInteractiveAvailable)
    (Rendering|Material|SetOverlayMaterial (Variables|Default|GetSM_FuseBox_Body) "/Game/content_2/InteractiveObject/Effects/MI_Outline.MI_Outline" :!class /Script/Engine.MeshComponent)
    (Rendering|Material|SetOverlayMaterial (Variables|Default|GetSM_FuseBox_Door) "/Game/content_2/InteractiveObject/Effects/MI_Outline.MI_Outline" :!class /Script/Engine.MeshComponent)))

(event EventOnHoverEnd
  (Rendering|Material|SetOverlayMaterial (Variables|Default|GetSM_FuseBox_Body) 0 :!class /Script/Engine.MeshComponent)
  (Rendering|Material|SetOverlayMaterial (Variables|Default|GetSM_FuseBox_Door) 0 :!class /Script/Engine.MeshComponent))

(event EventDoMainAction
  (params (HitResult :type Hit%20Result%20Structure))
  (bind _sm_fusebox_door (Variables|Default|GetSM_FuseBox_Door))
  (Variables|Default|SetInteractiveAvailable false)
  (Utilities|FlowControl|Sequence
    (:then_0
      (Rendering|Material|SetOverlayMaterial (Variables|Default|GetSM_FuseBox_Body) 0 :!class /Script/Engine.MeshComponent)
      (Rendering|Material|SetOverlayMaterial (Variables|Default|GetSM_FuseBox_Door) 0 :!class /Script/Engine.MeshComponent))
    (:then_1
      (Components|Activation|Activate (Variables|Default|GetP_Sparks_E) false)
      (Components|Activation|Activate (Variables|Default|GetP_Sparks_F) false)
      (Utilities|FlowControl|Delay 0.8)
      (Components|Activation|Deactivate (Variables|Default|GetP_Sparks_E))
      (Components|Activation|Deactivate (Variables|Default|GetP_Sparks_F)))
    (:then_2
      (Physics|SetSimulatePhysics _sm_fusebox_door true)
      (Physics|AddImpulse _sm_fusebox_door (* (Math|Random|RandomUnitVector) "500.000000,500.000000,50.000000") "None" false)
      (bind _outactors (Collision|SphereOverlapActors (Transformation|GetActorLocation) 3e+02 (Utilities|Array|MakeArray "ObjectTypeQuery1" "ObjectTypeQuery3") "/Game/content_1/scripts/ai/characters/humans/character_enemy_doctor.character_enemy_doctor_C"))
      (bind _ascharacter_enemy_doctor (Utilities|Casting|CastTocharacter_enemy_doctor (Utilities|Array|Get(acopy) _outactors)))
      (Default|HCFuseBoxReaction _ascharacter_enemy_doctor (Transformation|GetActorLocation)))))

(fn ConstructionScript)

(fn IsFocusAvailable
  (return false))

(fn IsInteractionAvailable
  (return (Variables|Default|GetInteractiveAvailable)))

(fn IsMainActionAvailable
  (return true))

(fn IsMainHoldActionAvailable
  (return false))

(fn IsSecondActionAvailable
  (return false))

(fn IsSecondHoldActionAvailable
  (return false))
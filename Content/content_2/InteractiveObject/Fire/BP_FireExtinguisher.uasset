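; BP_FireExtinguisher is a one-shot interactive fire extinguisher that outlines on hover and bursts when used.
; The main action starts a child-actor smoke effect, plays sounds and flings the three mesh parts with physics and random impulses.
; A sphere overlap then triggers a reaction on the first nearby enemy doctor found.
; The construction script uses OnWall to position the smoke, hiding the sign and rotating the body for floor placement.
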(event EventOnHoverStart
  (if (Variables|Default|GetbIsActionAvailable)
    (Rendering|Material|SetOverlayMaterial (Variables|Default|GetFireExtinguisher_Body) "/Game/content_2/InteractiveObject/Effects/MI_Outline.MI_Outline" :!class /Script/Engine.MeshComponent)))

(event EventOnHoverEnd
  (Rendering|Material|SetOverlayMaterial (Variables|Default|GetFireExtinguisher_Body) 0 :!class /Script/Engine.MeshComponent))

(event EventDoMainAction
  (params (HitResult :type Hit%20Result%20Structure))
  (bind _returnvalue (Math|Random|RandomUnitVector))
  (bind _fireextinguisher_body (Variables|Default|GetFireExtinguisher_Body))
  (bind _returnvalue_2 (* _returnvalue "500.000000,500.000000,50.000000"))
  (Utilities|FlowControl|DoOnce false
    (:Completed
      (Variables|Default|SetbIsActionAvailable false)
      (bind _asbp_vdb_smoke (Utilities|Casting|CastToBP_VDB_Smoke (Variables|/Script/Engine.ChildActorComponent|GetChildActor (Variables|Default|GetSmoke))))
      (Default|Start _asbp_vdb_smoke)
      (Audio|PlaySound2D "/Game/content_2/PlayerAuraEffect/Audio/Sounds_Cue/A_DashWoosh04_Cue.A_DashWoosh04_Cue" 1.0 1.0 0.0 0 0)
      (Audio|PlaySound2D "/Game/content_2/Doors_And_Drawers_SFX/Metal/WAW_Metal_Ring.WAW_Metal_Ring" 1.0 1.0 0.0 0 0)
      (Physics|SetSimulatePhysics _fireextinguisher_body true)
      (Class|PrimitiveComponent|AddAngularImpulseinDegrees _fireextinguisher_body _returnvalue_2 "None" true)
      (Physics|AddImpulse _fireextinguisher_body _returnvalue_2 "None" true)
      (bind _outactors (Collision|SphereOverlapActors (Transformation|GetActorLocation) 3e+02 (Utilities|Array|MakeArray "ObjectTypeQuery1" "ObjectTypeQuery3") "/Game/content_1/scripts/ai/characters/humans/character_enemy_doctor.character_enemy_doctor_C"))
      (bind _ascharacter_enemy_doctor (Utilities|Casting|CastTocharacter_enemy_doctor (Utilities|Array|Get(acopy) _outactors)))
      (Default|HCFireExstReaction _ascharacter_enemy_doctor))))

(fn ConstructionScript
  (bind _smoke (Variables|Default|GetSmoke))
  (bind _smoke_2 (Variables|Default|GetSmoke))
  (if (Variables|Default|GetbOnWall)
    (Transformation|SetRelativeLocation _smoke (Variables|Default|GetOnWallLocation) false false)
    (Transformation|SetRelativeRotation _smoke "90.000000,0.000000,0.000000" false false)
    (else
      (Transformation|SetRelativeLocation _smoke_2 (Variables|Default|GetOnFloorLocation) false false)
      (Transformation|SetRelativeRotation _smoke_2 "0, 0, 0" false false)
      (Transformation|SetRelativeRotation (Variables|Default|GetFireExtinguisher_Body) "90.000000,0.000000,0.000000" false false)
      (Rendering|SetVisibility (Variables|Default|GetSign) false false))))

(fn IsFocusAvailable
  (return false))

(fn IsInteractionAvailable
  (return true))

(fn IsMainActionAvailable
  (return true))

(fn IsMainHoldActionAvailable
  (return false))

(fn IsSecondActionAvailable
  (return false))

(fn IsSecondHoldActionAvailable
  (return false))
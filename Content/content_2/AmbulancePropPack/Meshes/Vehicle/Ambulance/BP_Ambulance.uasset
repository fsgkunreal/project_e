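; Configurable ambulance prop whose look and pose are set entirely in the Construction Script, with no active runtime logic.
; Exposes variables for cab and shell materials, Dents and Dust material parameters, front wheel steering, wheel heights, hinged door rotations and interior sliding door offsets.
; Spawns two LicensePlate child actors and copies the first plate's six character meshes onto the second so both match.
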(event EventBeginPlay)

(event Collision|EventActorBeginOverlap
  (params (OtherActor :type Actor%20Object%20Reference)))

(event EventTick
  (params (DeltaSeconds :type Float%20%28single-precision%29)))

(fn ConstructionScript
  (bind _ambulance (Variables|Default|GetAmbulance))
  (bind _shell_right_small_rear_door (Variables|Default|GetShell%20Right%20Small%20Rear%20Door))
  (bind _left_front_wheel (Variables|Default|GetLeft%20Front%20Wheel))
  (bind _right_front_wheel (Variables|Default|GetRight%20Front%20Wheel))
  (bind _front_wheels_rotation (Variables|DoorControl|GetFront%20Wheels%20Rotation))
  (bind _interior_sliding_door_1 (Variables|Default|GetInterior%20Sliding%20Door%201))
  (bind _interior_sliding_door_2 (Variables|Default|GetInterior%20Sliding%20Door%202))
  (bind _interior_sliding_door_3 (Variables|Default|GetInterior%20Sliding%20Door%203))
  (bind _interior_sliding_door_4 (Variables|Default|GetInterior%20Sliding%20Door%204))
  (bind _cab_material (Variables|Material|GetCab%20Material))
  (bind _interior_sliding_door_5 (Variables|Default|GetInterior%20Sliding%20Door%205))
  (bind _interior_sliding_door_6 (Variables|Default|GetInterior%20Sliding%20Door%206))
  (bind _interior_sliding_door_7 (Variables|Default|GetInterior%20Sliding%20Door%207))
  (bind _rear_right_wheel (Variables|Default|GetRear%20Right%20Wheel))
  (bind _rear_left_wheel (Variables|Default|GetRear%20Left%20Wheel))
  (bind _shell_material (Variables|Material|GetShell%20Material))
  (bind _cab_left_door (Variables|Default|GetCab%20Left%20Door))
  (bind _cab_right_door (Variables|Default|GetCab%20Right%20Door))
  (bind _relativelocation (Variables|/Script/Engine.SceneComponent|GetRelativeLocation _interior_sliding_door_7))
  (bind _relativelocation_2 (Variables|/Script/Engine.SceneComponent|GetRelativeLocation _rear_left_wheel))
  (bind _relativelocation_3 (Variables|/Script/Engine.SceneComponent|GetRelativeLocation _interior_sliding_door_2))
  (bind _relativelocation_4 (Variables|/Script/Engine.SceneComponent|GetRelativeLocation _interior_sliding_door_3))
  (bind _relativelocation_5 (Variables|/Script/Engine.SceneComponent|GetRelativeLocation _interior_sliding_door_4))
  (bind _relativelocation_6 (Variables|/Script/Engine.SceneComponent|GetRelativeLocation _interior_sliding_door_5))
  (bind _relativelocation_7 (Variables|/Script/Engine.SceneComponent|GetRelativeLocation _interior_sliding_door_6))
  (bind _relativelocation_8 (Variables|/Script/Engine.SceneComponent|GetRelativeLocation _interior_sliding_door_1))
  (bind _relativelocation_9 (Variables|/Script/Engine.SceneComponent|GetRelativeLocation _right_front_wheel))
  (bind _relativelocation_10 (Variables|/Script/Engine.SceneComponent|GetRelativeLocation _rear_right_wheel))
  (bind _relativelocation_11 (Variables|/Script/Engine.SceneComponent|GetRelativeLocation _left_front_wheel))
  (bind (_x _y _z) (Math|Vector|BreakVector _relativelocation))
  (bind (_x_2 _y_2) (Math|Vector|BreakVector _relativelocation_2))
  (bind (_x_3 _y_3 _z_2) (Math|Vector|BreakVector _relativelocation_3))
  (bind (_x_4 _y_4 _z_3) (Math|Vector|BreakVector _relativelocation_4))
  (bind (_x_5 _y_5 _z_4) (Math|Vector|BreakVector _relativelocation_5))
  (bind (_x_6 _y_6 _z_5) (Math|Vector|BreakVector _relativelocation_6))
  (bind (_x_7 _y_7 _z_6) (Math|Vector|BreakVector _relativelocation_7))
  (bind (_x_8 _y_8 _z_7) (Math|Vector|BreakVector _relativelocation_8))
  (bind (_x_9 _y_9) (Math|Vector|BreakVector _relativelocation_9))
  (bind (_x_10 _y_10) (Math|Vector|BreakVector _relativelocation_10))
  (bind (_x_11 _y_11) (Math|Vector|BreakVector _relativelocation_11))
  ;[0.09042 0.5677 0.1213 1 15] Cab & Shell Matswap
  (Rendering|Material|SetMaterial _ambulance 3 _cab_material)
  (Rendering|Material|SetMaterial _ambulance 2 _shell_material)
  (Rendering|Material|SetMaterial (Variables|Default|GetBumper) 0 _cab_material)
  (Rendering|Material|SetMaterial _cab_left_door 2 _cab_material)
  (Rendering|Material|SetMaterial _cab_right_door 0 _cab_material)
  (Rendering|Material|SetMaterial _shell_right_small_rear_door 0 _shell_material)
  ;[0.09042 0.5677 0.1213 1 15] Dents Slider
  (Rendering|Material|SetScalarParameterValueonMaterials _ambulance "Dents" (Variables|Material|GetDents))
  ;[0.09042 0.5677 0.1213 1 15] Dust Slider
  (Rendering|Material|SetScalarParameterValueonMaterials _cab_right_door "Dust" (Variables|Material|GetDust))
  ;[0.5571 0.4992 0.8958 1 15] Front Wheel Rotation
  (Transformation|SetRelativeRotation _left_front_wheel (Math|Rotator|MakeRotator 0.0 0.0 _front_wheels_rotation) false false)
  (Transformation|SetRelativeRotation _right_front_wheel (Math|Rotator|MakeRotator 0.0 0.0 (+ _front_wheels_rotation 1.8e+02)) false false)
  ;[0.5571 0.4992 0.8958 1 15] Left Door Rotation
  (Transformation|SetRelativeRotation _cab_left_door (Math|Rotator|MakeRotator 0.0 0.0 (Variables|DoorControl|GetCab%20Left%20Door%20Rotation)) false false)
  ;[0.5571 0.4992 0.8958 1 15] Right Door Rotation
  (Transformation|SetRelativeRotation _cab_right_door (Class|KismetMathLibrary|NegateRotator (Math|Rotator|MakeRotator 0.0 0.0 (Variables|DoorControl|GetCab%20Right%20Door%20Rotation))) false false)
  ;[0.9301 0.552 0.016 1 15] Wheel Z Adjustment
  (Transformation|SetRelativeLocation _right_front_wheel (Math|Vector|MakeVector _x_9 _y_9 (Variables|WheelCorrection|GetFront%20Right%20Wheel%20Z)) false false)
  (Transformation|SetRelativeLocation _rear_right_wheel (Math|Vector|MakeVector _x_10 _y_10 (Variables|WheelCorrection|GetRear%20Right%20Wheel%20Z)) false false)
  (Transformation|SetRelativeLocation _left_front_wheel (Math|Vector|MakeVector _x_11 _y_11 (Variables|WheelCorrection|GetFront%20Left%20Wheel%20Z)) false false)
  (Transformation|SetRelativeLocation _rear_left_wheel (Math|Vector|MakeVector _x_2 _y_2 (Variables|WheelCorrection|GetRear%20Left%20Wheel%20Z)) false false)
  ;[0.5571 0.4992 0.8958 1 15] Ambulance Door Side Exit
  (Transformation|SetRelativeRotation (Variables|Default|GetShell%20Right%20Door%20Street%20Exit) (Class|KismetMathLibrary|NegateRotator (Math|Rotator|MakeRotator 0.0 0.0 (Variables|DoorControl|GetStreet%20Exit%20Door%20Rotation))) false false)
  ;[0.5571 0.4992 0.8958 1 15] Ambulance Rear Left Door Rotation
  (Transformation|SetRelativeRotation (Variables|Default|GetShell%20Rear%20Door%20Exit%20Left) (Math|Rotator|MakeRotator 0.0 0.0 (Variables|DoorControl|GetLeft%20Exit%20Door%20Rotation)) false false)
  ;[0.5571 0.4992 0.8958 1 15] Ambulance Rear Right Door Rotation
  (Transformation|SetRelativeRotation (Variables|Default|GetShell%20Rear%20Door%20Exit%20Right) (Class|KismetMathLibrary|NegateRotator (Math|Rotator|MakeRotator 0.0 0.0 (Variables|DoorControl|GetRight%20Exit%20Door%20Rotation))) false false)
  ;[0.5571 0.4992 0.8958 1 15] Shell Left Double Door 1
  (Transformation|SetRelativeRotation (Variables|Default|GetShell%20Left%20Double%20Door%201) (Math|Rotator|MakeRotator 0.0 0.0 (Variables|DoorControl|GetLeft%20Side%20Double%20Door%20L1%20Rotation)) false false)
  ;[0.5571 0.4992 0.8958 1 15] Shell Left Double Door 2
  (Transformation|SetRelativeRotation (Variables|Default|GetShell%20Left%20Double%20Door%202) (Class|KismetMathLibrary|NegateRotator (Math|Rotator|MakeRotator 0.0 0.0 (Variables|DoorControl|GetLeft%20Side%20Double%20Door%20R2%20Rotation))) false false)
  ;[0.5571 0.4992 0.8958 1 15] Stretcher Door
  (Transformation|SetRelativeRotation (Variables|Default|GetShell%20Right%20Stretcher%20Door) (Class|KismetMathLibrary|NegateRotator (Math|Rotator|MakeRotator 0.0 0.0 (Variables|DoorControl|GetStretcher%20Door%20Rotation))) false false)
  ;[0.5571 0.4992 0.8958 1 15] Small Door Rear Left
  (Transformation|SetRelativeRotation (Variables|Default|GetShell%20Left%20Small%20Rear%20Door) (Math|Rotator|MakeRotator 0.0 0.0 (Variables|DoorControl|GetLeft%20Side%20Small%20Door)) false false)
  ;[0.5571 0.4992 0.8958 1 15] Small Door Rear Right
  (Transformation|SetRelativeRotation _shell_right_small_rear_door (Class|KismetMathLibrary|NegateRotator (Math|Rotator|MakeRotator 0.0 0.0 (Variables|DoorControl|GetRight%20Side%20Small%20Door))) false false)
  ;[0.5571 0.4992 0.8958 1 15] Rear Compartment Left
  (Transformation|SetRelativeRotation (Variables|Default|GetShell%20Rear%20Side%20Door%20Left) (Math|Rotator|MakeRotator 0.0 0.0 (Variables|DoorControl|GetRear%20Compartment%20Left%20Door)) false false)
  ;[0.5571 0.4992 0.8958 1 15] Rear Compartment Right
  (Transformation|SetRelativeRotation (Variables|Default|GetShell%20Rear%20Side%20Door%20Right) (Class|KismetMathLibrary|NegateRotator (Math|Rotator|MakeRotator 0.0 0.0 (Variables|DoorControl|GetRear%20Compartment%20Right%20Door))) false false)
  ;[0.9301 0.552 0.016 1 15] Interior Compartment Sliding Doors
  (Transformation|SetRelativeLocation _interior_sliding_door_1 (Math|Vector|MakeVector (Variables|DoorControl-Interior|GetInterior%20Slide%20Door%201) _y_8 _z_7) false false)
  (Transformation|SetRelativeLocation _interior_sliding_door_2 (Math|Vector|MakeVector (Variables|DoorControl-Interior|GetInterior%20Slide%20Door%202) _y_3 _z_2) false false)
  (Transformation|SetRelativeLocation _interior_sliding_door_3 (Math|Vector|MakeVector (Variables|DoorControl-Interior|GetInterior%20Slide%20Door%203) _y_4 _z_3) false false)
  (Transformation|SetRelativeLocation _interior_sliding_door_4 (Math|Vector|MakeVector _x_5 (Variables|DoorControl-Interior|GetInterior%20Slide%20Door%204) _z_4) false false)
  (Transformation|SetRelativeLocation _interior_sliding_door_5 (Math|Vector|MakeVector _x_6 (Variables|DoorControl-Interior|GetInterior%20Slide%20Door%205) _z_5) false false)
  (Transformation|SetRelativeLocation _interior_sliding_door_6 (Math|Vector|MakeVector (Variables|DoorControl-Interior|GetInterior%20Slide%20Door%206) _y_7 _z_6) false false)
  (Transformation|SetRelativeLocation _interior_sliding_door_7 (Math|Vector|MakeVector (Variables|DoorControl-Interior|GetInterior%20Slide%20Door%207) _y _z) false false)
  ;[0 0.3645 1] License Plate
  (bind _returnvalue (AddComponent|AddChildActorComponent false (Math|Transform|MakeTransform "356.600006,55.400002,55.400002" "0,180.000000, 0" "1.000000,1.000000,1.000000")))
  (bind _aslicense_plate (Utilities|Casting|CastToLicensePlate (Variables|/Script/Engine.ChildActorComponent|GetChildActor _returnvalue)))
  (bind _returnvalue_2 (AddComponent|AddChildActorComponent false (Math|Transform|MakeTransform (Variables|LicensePlate|GetLicense%20Plate%20Position) "12.000000, 0,0.000000" "1.000000,1.000000,1.000000")))
  (bind _aslicense_plate_2 (Utilities|Casting|CastToLicensePlate (Variables|/Script/Engine.ChildActorComponent|GetChildActor _returnvalue_2)))
  (Components|StaticMesh|SetStaticMesh (Variables|/Game/content_2/AmbulancePropPack/Meshes/Vehicle/LicensePlate/LicensePlate.LicensePlate_C|Get0 _aslicense_plate_2) (Variables|/Game/content_2/AmbulancePropPack/Meshes/Vehicle/LicensePlate/LicensePlate.LicensePlate_C|Get0%20spot _aslicense_plate))
  (Components|StaticMesh|SetStaticMesh (Variables|/Game/content_2/AmbulancePropPack/Meshes/Vehicle/LicensePlate/LicensePlate.LicensePlate_C|Get1 _aslicense_plate_2) (Variables|/Game/content_2/AmbulancePropPack/Meshes/Vehicle/LicensePlate/LicensePlate.LicensePlate_C|Get1%20Spot _aslicense_plate))
  (Components|StaticMesh|SetStaticMesh (Variables|/Game/content_2/AmbulancePropPack/Meshes/Vehicle/LicensePlate/LicensePlate.LicensePlate_C|Get2 _aslicense_plate_2) (Variables|/Game/content_2/AmbulancePropPack/Meshes/Vehicle/LicensePlate/LicensePlate.LicensePlate_C|Get2%20Spot _aslicense_plate))
  (Components|StaticMesh|SetStaticMesh (Variables|/Game/content_2/AmbulancePropPack/Meshes/Vehicle/LicensePlate/LicensePlate.LicensePlate_C|Get3 _aslicense_plate_2) (Variables|/Game/content_2/AmbulancePropPack/Meshes/Vehicle/LicensePlate/LicensePlate.LicensePlate_C|Get3%20Spot _aslicense_plate))
  (Components|StaticMesh|SetStaticMesh (Variables|/Game/content_2/AmbulancePropPack/Meshes/Vehicle/LicensePlate/LicensePlate.LicensePlate_C|Get4 _aslicense_plate_2) (Variables|/Game/content_2/AmbulancePropPack/Meshes/Vehicle/LicensePlate/LicensePlate.LicensePlate_C|Get4%20Spot _aslicense_plate))
  (Components|StaticMesh|SetStaticMesh (Variables|/Game/content_2/AmbulancePropPack/Meshes/Vehicle/LicensePlate/LicensePlate.LicensePlate_C|Get5 _aslicense_plate_2) (Variables|/Game/content_2/AmbulancePropPack/Meshes/Vehicle/LicensePlate/LicensePlate.LicensePlate_C|Get5%20Spot _aslicense_plate)))
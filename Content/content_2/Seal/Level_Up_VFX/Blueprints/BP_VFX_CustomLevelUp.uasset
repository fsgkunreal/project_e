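; Demo actor that repeatedly plays a customizable level-up effect at its location, alongside a color picker widget toggled with H.
; Each looped UseAbility spawns a base Niagara system, floating screen text and optional arrows, ground and sparkles chosen in the widget.
; A Fresnel timeline animates emissive in MPC_CustomColor, whose two colors the construction script sets.
; The looping PlaySound event is never called.
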(event Custom|UseAbility
  (bind _widget (Variables|Default|GetWidget))
  ;[0.252 0.5038 1] SPAWN VFX
  (Utilities|FlowControl|Sequence
    (:then_0
      (Variables|Default|SetaddGround (Variables|/Game/content_2/Seal/Level_Up_VFX/UI/ColorPickerVFX_HSV.ColorPickerVFX_HSV_C|GetuseGround _widget))
      (Variables|Default|SetaddSparkles (Variables|/Game/content_2/Seal/Level_Up_VFX/UI/ColorPickerVFX_HSV.ColorPickerVFX_HSV_C|GetuseSparkles _widget))
      (Variables|Default|SetaddArrows (Variables|/Game/content_2/Seal/Level_Up_VFX/UI/ColorPickerVFX_HSV.ColorPickerVFX_HSV_C|GetuseArrows _widget)))
    (:then_1
      (Utilities|FlowControl|Sequence
        (:then_0
          (bind _returnvalue (Niagara|SpawnSystematLocation "/Game/content_2/Seal/Level_Up_VFX/Shared/Particles/NS_Level_Up_Base_Test.NS_Level_Up_Base_Test" (Transformation|GetActorLocation) (Transformation|GetActorRotation)))
          (Variables|Default|SetCurrentVFX _returnvalue)
          (Utilities|FlowControl|Sequence
            (:then_0
              (Utilities|FlowControl|RetriggerableDelay (Variables|Default|GetDelaySpawnFX))
              (CallFunction|UseAbility))
            (:then_1
              (bind _emissive (Timeline|Fresnel PlayFromStart)
                (:Update
                  (Rendering|Material|SetScalarParameterValue "/Game/content_2/Seal/Level_Up_VFX/Shared/Materials/MPC_CustomColor.MPC_CustomColor" "Fresnel_Emissive" _emissive :!class /Script/Engine.KismetMaterialLibrary))))
            (:then_2
              (CallFunction|SpawnLvlUpText (+ (Transformation|GetWorldLocation (Variables|Default|GetDefaultSceneRoot)) "0, 0,200.000000")))))
        (:then_1
          (if (Variables|Default|GetaddArrows)
            (Niagara|SpawnSystematLocation "/Game/content_2/Seal/Level_Up_VFX/Shared/Particles/NS_Level_Up_Arrows_Test.NS_Level_Up_Arrows_Test" (Transformation|GetActorLocation) (Transformation|GetActorRotation))))
        (:then_2
          (if (Variables|Default|GetaddGround)
            (Niagara|SpawnSystematLocation "/Game/content_2/Seal/Level_Up_VFX/Shared/Particles/NS_Level_Up_Ground_Test.NS_Level_Up_Ground_Test" (Transformation|GetActorLocation) (Transformation|GetActorRotation))))
        (:then_3
          (if (Variables|Default|GetaddSparkles)
            (Niagara|SpawnSystematLocation "/Game/content_2/Seal/Level_Up_VFX/Shared/Particles/NS_Level_Up_Sparkles_Test.NS_Level_Up_Sparkles_Test" (Transformation|GetActorLocation) (Transformation|GetActorRotation))))))))

(event Custom|PlaySound
  (bind _returnvalue (Audio|SpawnSoundatLocation (Utilities|Array|Get(acopy) (Variables|SoundsList|GetSFX%20List) (Variables|Default|GetElementList)) (Transformation|GetWorldLocation (Variables|Default|GetProjectileOffset)) "0, 0, 0" 1.0 1.0 0.0 0 0))
  (Variables|Default|SetCurrentSFX _returnvalue)
  (Utilities|FlowControl|RetriggerableDelay 0.2)
  (CallFunction|PlaySound))

(event Custom|Spawn%20Lvl%20Up%20Text
  (params (WorldPos :type Vector))
  (bind _returnvalue (Game|GetPlayerController 0))
  ;[0.252 0.5038 1] SPAWN VFX
  (bind _returnvalue_2 (UserInterface|CreateWidget "/Game/content_2/Seal/Level_Up_VFX/UI/FloatingText_LvlUp.FloatingText_LvlUp_C" _returnvalue (.ScreenPosition (Class|WidgetLayoutLibrary|ProjectWorldLocationtoWidgetPosition _returnvalue WorldPos false))))
  (UserInterface|Viewport|AddtoViewport _returnvalue_2 0))

(event EventBeginPlay
  (Utilities|FlowControl|Sequence
    (:then_0
      ;[0.5326 1 0.2247] UI Color Picker
      (bind _returnvalue (UserInterface|CreateWidget "/Game/content_2/Seal/Level_Up_VFX/UI/ColorPickerVFX_HSV.ColorPickerVFX_HSV_C"))
      (bind _output_get (Variables|Default|SetWidget _returnvalue))
      (UserInterface|Viewport|AddtoViewport _output_get 0))
    (:then_1
      (Input|EnableInput (Game|GetPlayerController 0)))
    (:then_2
      (CallFunction|UseAbility))))

(event Input|KeyboardEvents|H
  (params (Key :type Key%20Structure))
  (bind _widget (Variables|Default|GetWidget))
  (:Pressed
    (Utilities|FlowControl|FlipFlop
      (:A
        (Widget|SetVisibility _widget "Hidden"))
      (:B
        (Widget|SetVisibility _widget "Visible")))))

(fn ConstructionScript
  (Rendering|Material|SetVectorParameterValue "/Game/content_2/Seal/Level_Up_VFX/Shared/Materials/MPC_CustomColor.MPC_CustomColor" "Color_01" (Variables|Default|GetColor_01) :!class /Script/Engine.KismetMaterialLibrary)
  (Rendering|Material|SetVectorParameterValue "/Game/content_2/Seal/Level_Up_VFX/Shared/Materials/MPC_CustomColor.MPC_CustomColor" "Color_02" (Variables|Default|GetColor_02) :!class /Script/Engine.KismetMaterialLibrary))
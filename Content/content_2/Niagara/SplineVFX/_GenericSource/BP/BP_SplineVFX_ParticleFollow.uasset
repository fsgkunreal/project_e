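; Spline VFX actor that drives a Niagara effect's Progress over time, named as a particle-follow effect.
; The construction script rebuilds an open local-space spline from points on a flat circle, using an inverted degree-to-radian conversion that winds it around several times.
; It also sets the Timeline play rate from GrowSpeed.
; On BeginPlay, the Timeline plays from start and feeds its track into Progress each update.
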(event EventBeginPlay
  (bind _newtrack_0 (Timeline|Timeline PlayFromStart)
    (:Update
      (Niagara|SetNiagaraVariable(Float) (Variables|Default|GetNiagara) "Progress" _newtrack_0))))

(event Collision|EventActorBeginOverlap
  (params (OtherActor :type Actor%20Object%20Reference)))

(fn ConstructionScript
  (bind _spline (Variables|Default|GetSpline))
  (Utilities|FlowControl|Sequence
    (:then_0
      (Spline|ClearSplinePoints _spline true)
      (for _index (range 0 31)
        (Spline|AddSplinePoint _spline (Math|Vector|MakeVector (* (Math|Trig|Cos(Radians) (* (* (/ (Math|Conversions|ToFloat(Integer) _index) 31.0) 3.6e+02) (/ 1.8e+02 (Math|Float|MultiplybyPi 1.0)))) 5e+01) (* (Math|Trig|Sin(Radians) (* (* (/ (Math|Conversions|ToFloat(Integer) _index) 31.0) 3.6e+02) (/ 1.8e+02 (Math|Float|MultiplybyPi 1.0)))) 5e+01) 0.0) "Local" true))
      (Spline|SetClosedLoop _spline false true))
    (:then_1
      (Components|Timeline|SetPlayRate (Variables|Default|GetTimeline) (Variables|Default|GetGrowSpeed)))))
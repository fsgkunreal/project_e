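; Placeable VDB smoke actor that plays one of ten animated smoke variants through a Heterogeneous Volume.
; The construction script applies playback, scale and optional snap to Z=0, then sets each variant's material and offset, updating frame rate for the first two after it is applied.
; Density and color go to a shared Material Parameter Collection, affecting all instances.
; A Start event plays the volume unlooped from a fixed frame.
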(event Custom|Start
  (bind _heterogeneousvolume (Variables|Default|GetHeterogeneousVolume))
  (Components|Timeline|SetLooping _heterogeneousvolume false)
  (Class|HeterogeneousVolumeComponent|SetFrame _heterogeneousvolume 6e+01)
  (Class|HeterogeneousVolumeComponent|SetPlaying _heterogeneousvolume true))

(event EventBeginPlay
  (if (Variables|Default|GetActivateSmoke)
    (Utilities|FlowControl|DoOnce false)))

(event Collision|EventActorBeginOverlap
  (params (OtherActor :type Actor%20Object%20Reference)))

(event EventTick
  (params (DeltaSeconds :type Float%20%28single-precision%29)))

(fn ConstructionScript
  (bind _returnvalue (Transformation|GetActorTransform))
  (bind _heterogeneousvolume (Variables|Default|GetHeterogeneousVolume))
  (bind _heterogeneousvolume_2 (Variables|Default|GetHeterogeneousVolume))
  (bind _heterogeneousvolume_3 (Variables|Default|GetHeterogeneousVolume))
  (bind _heterogeneousvolume_4 (Variables|Default|GetHeterogeneousVolume))
  (bind _heterogeneousvolume_5 (Variables|Default|GetHeterogeneousVolume))
  (bind _heterogeneousvolume_6 (Variables|Default|GetHeterogeneousVolume))
  (bind _heterogeneousvolume_7 (Variables|Default|GetHeterogeneousVolume))
  (bind _heterogeneousvolume_8 (Variables|Default|GetHeterogeneousVolume))
  (bind _heterogeneousvolume_9 (Variables|Default|GetHeterogeneousVolume))
  (bind _heterogeneousvolume_10 (Variables|Default|GetHeterogeneousVolume))
  (bind _heterogeneousvolume_11 (Variables|Default|GetHeterogeneousVolume))
  (if (Variables|Default|GetDoOnce)
    (Utilities|FlowControl|DoOnce false
      (:Completed
        (Variables|Playing|SetPlaying true)
        (Variables|Playing|SetLooping false))))
  (Utilities|FlowControl|Sequence
    (:then_0
      ;[0 0 0] PlayingSettings
      (Components|Timeline|SetLooping _heterogeneousvolume (Variables|Playing|GetLooping))
      (Class|HeterogeneousVolumeComponent|SetPlaying _heterogeneousvolume (Variables|Playing|GetPlaying))
      (Class|HeterogeneousVolumeComponent|SetFrame _heterogeneousvolume (Variables|Playing|GetFrame))
      (Class|HeterogeneousVolumeComponent|SetFrameRate _heterogeneousvolume (Variables|Playing|GetFrameRate%28FPS%29)))
    (:then_1
      ;[0 0 0] Scale
      (Transformation|SetWorldScale3D (Variables|Default|GetCenter) (Variables|Pos/Scale|GetSetScale)))
    (:then_2
      (if (Variables|Pos/Scale|GetSnap_Ground_0Pos)
        (Transformation|SetActorTransform (Math|Transform|MakeTransform (Math|Vector|MakeVector (.x (.location _returnvalue)) (.y (.location _returnvalue)) 0.0) (.rotation _returnvalue) (.scale _returnvalue)))))
    (:then_3
      ;[0 0 0] SetMaterial / Position
      (switch Utilities|FlowControl|Switch|SwitchonEnum_SmokeFxList (Variables|SmokeStyle|GetEnum_SmokeTypes)
        (:NewEnumerator0
          (Rendering|Material|SetMaterial _heterogeneousvolume_7 0 "/Game/content_2/SmokePack/Sources/Materials/Instance/MI_VdbSmoke_01.MI_VdbSmoke_01")
          (Transformation|SetRelativeLocation _heterogeneousvolume_7 "-4.835247,-54.231038,63.149012" false false)
          (Variables|Playing|SetFrameRate%28FPS%29 6e+01))
        (:NewEnumerator1
          (Rendering|Material|SetMaterial _heterogeneousvolume_2 0 "/Game/content_2/SmokePack/Sources/Materials/Instance/MI_VdbSmoke_02.MI_VdbSmoke_02")
          (Transformation|SetRelativeLocation _heterogeneousvolume_2 "0.000000,0.000000,110.314885" false false)
          (Variables|Playing|SetFrameRate%28FPS%29 3e+01))
        (:NewEnumerator2
          (Rendering|Material|SetMaterial _heterogeneousvolume_9 0 "/Game/content_2/SmokePack/Sources/Materials/Instance/MI_VdbSmoke_03.MI_VdbSmoke_03")
          (Transformation|SetRelativeLocation _heterogeneousvolume_9 "0.000000,0.000000,110.314885" false false))
        (:NewEnumerator3
          (Rendering|Material|SetMaterial _heterogeneousvolume_10 0 "/Game/content_2/SmokePack/Sources/Materials/Instance/MI_VdbSmoke_04.MI_VdbSmoke_04")
          (Transformation|SetRelativeLocation _heterogeneousvolume_10 "0.000000,0.000000,60.000000" false false))
        (:NewEnumerator4
          (Rendering|Material|SetMaterial _heterogeneousvolume_11 0 "/Game/content_2/SmokePack/Sources/Materials/Instance/MI_VdbSmoke_05.MI_VdbSmoke_05")
          (Transformation|SetRelativeLocation _heterogeneousvolume_11 "0.000000,0.000000,86.000000" false false))
        (:NewEnumerator5
          (Rendering|Material|SetMaterial _heterogeneousvolume_3 0 "/Game/content_2/SmokePack/Sources/Materials/Instance/MI_VdbSmoke_06.MI_VdbSmoke_06")
          (Transformation|SetRelativeLocation _heterogeneousvolume_3 "0.000000,0.000000,101.000000" false false))
        (:NewEnumerator6
          (Rendering|Material|SetMaterial _heterogeneousvolume_4 0 "/Game/content_2/SmokePack/Sources/Materials/Instance/MI_VdbSmoke_07.MI_VdbSmoke_07")
          (Transformation|SetRelativeLocation _heterogeneousvolume_4 "0.000000,0.000000,60.000000" false false))
        (:NewEnumerator7
          (Rendering|Material|SetMaterial _heterogeneousvolume_5 0 "/Game/content_2/SmokePack/Sources/Materials/Instance/MI_VdbSmoke_08.MI_VdbSmoke_08")
          (Transformation|SetRelativeLocation _heterogeneousvolume_5 "0.000000,0.000000,70.000000" false false))
        (:NewEnumerator8
          (Rendering|Material|SetMaterial _heterogeneousvolume_6 0 "/Game/content_2/SmokePack/Sources/Materials/Instance/MI_VdbSmoke_09.MI_VdbSmoke_09")
          (Transformation|SetRelativeLocation _heterogeneousvolume_6 "0.000000,0.000000,160.659218" false false))
        (:NewEnumerator9
          (Rendering|Material|SetMaterial _heterogeneousvolume_8 0 "/Game/content_2/SmokePack/Sources/Materials/Instance/MI_VdbSmoke_10.MI_VdbSmoke_10")
          (Transformation|SetRelativeLocation _heterogeneousvolume_8 "0.000000,0.000000,86.000000" false false))))
    (:then_4
      ;[0 0 0] Material Parameters Control
      (Utilities|FlowControl|Sequence
        (:then_0
          (Rendering|Material|SetScalarParameterValue "/Game/content_2/SmokePack/Sources/Materials/MPC/MPC_VdbControl.MPC_VdbControl" "Density Scale" (Variables|MaterialControl|GetDensityScale) :!class /Script/Engine.KismetMaterialLibrary))
        (:then_1
          (Rendering|Material|SetVectorParameterValue "/Game/content_2/SmokePack/Sources/Materials/MPC/MPC_VdbControl.MPC_VdbControl" "Smoke Color" (Variables|MaterialControl|GetSmoke%20Color) :!class /Script/Engine.KismetMaterialLibrary))))))
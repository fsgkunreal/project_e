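; BP_Ceiling_Lamp is a ceiling lamp actor with a rect light, filed under the RoomEditor ceiling content.
; Its construction script multiplies the light's source width and height by the actor's Y and X scale respectively.
; The AdditionalIndirectLight flag selects a higher or lower indirect lighting intensity, and PlayerWard selects a brighter or dimmer light intensity.
; The event graph has no active logic.
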(event EventBeginPlay)

(event Collision|EventActorBeginOverlap
  (params (OtherActor :type Actor%20Object%20Reference)))

(event EventTick
  (params (DeltaSeconds :type Float%20%28single-precision%29)))

(fn ConstructionScript
  (bind _returnvalue (Transformation|GetActorScale3D))
  (bind _rectlight (Variables|Default|GetRectLight))
  (bind _rectlight_2 (Variables|Default|GetRectLight))
  (Class|RectLightComponent|SetSourceWidth _rectlight (* (Variables|/Script/Engine.RectLightComponent|GetSourceWidth _rectlight) (.y _returnvalue)))
  (Class|RectLightComponent|SetSourceHeight _rectlight (* (Variables|/Script/Engine.RectLightComponent|GetSourceHeight _rectlight) (.x _returnvalue)))
  (if (Variables|Default|GetAdditionalIndirectLight)
    (Class|LightComponent|SetIndirectLightingIntensity _rectlight_2 45.0)
    (else
      (Class|LightComponent|SetIndirectLightingIntensity _rectlight_2 2e+01)))
  (if (Variables|Default|GetPlayerWard)
    (Rendering|Components|Light|SetIntensity (Variables|Default|GetRectLight) 2.5e+02)
    (else
      (Rendering|Components|Light|SetIntensity (Variables|Default|GetRectLight) 1.8e+02))))
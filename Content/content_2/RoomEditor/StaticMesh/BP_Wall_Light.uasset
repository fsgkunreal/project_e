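; BP_Wall_Light is a room editor wall light actor with two rect lights, RectLightX and RectLightY, each toggled by its own visibility flag.
; The construction script applies SourceHeight to both lights and derives intensity, scaled by MaxIntensity, and attenuation radius from it, so longer sources shine brighter and reach farther.
; The event graph does nothing at runtime, holding only disconnected leftover nodes.
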(event EventBeginPlay)

(fn ConstructionScript
  (bind _maxintensity (Variables|Default|GetMaxIntensity))
  (bind _sourceheight (Variables|Default|GetSourceHeight))
  (bind _sourceheight_2 (Variables|Default|GetSourceHeight))
  (bind _sourceheight_3 (Variables|Default|GetSourceHeight))
  (bind _returnvalue (/ _sourceheight_3 1.5))
  (bind _returnvalue_2 (/ 1e+03 _maxintensity))
  (bind _returnvalue_3 (/ _sourceheight _returnvalue_2))
  (Class|RectLightComponent|SetSourceHeight (Variables|Default|GetRectLightY) _sourceheight_2)
  (Class|RectLightComponent|SetSourceHeight (Variables|Default|GetRectLightX) _sourceheight_2)
  (Rendering|Components|Light|SetIntensity (Variables|Default|GetRectLightY) _returnvalue_3)
  (Rendering|Components|Light|SetIntensity (Variables|Default|GetRectLightX) _returnvalue_3)
  (Rendering|Lighting|SetAttenuationRadius (Variables|Default|GetRectLightY) _returnvalue)
  (Rendering|Lighting|SetAttenuationRadius (Variables|Default|GetRectLightX) _returnvalue)
  (Rendering|SetVisibility (Variables|Default|GetRectLightX) (Variables|Default|GetRectVisibleX) false)
  (Rendering|SetVisibility (Variables|Default|GetRectLightY) (Variables|Default|GetRectVisibleY) false))
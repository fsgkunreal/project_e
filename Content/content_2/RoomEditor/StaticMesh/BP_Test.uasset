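; BP_Test is a test Blueprint that configures two rect lights from a shared source height.
; The construction script applies SourceHeight to both lights and scales their intensity linearly with it, reaching MaxIntensity at a height of 1000.
; BeginPlay is empty, and the event graph holds only unconnected leftovers: a copy of that logic and a call that zeroes intensity.
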(event EventBeginPlay)

(fn ConstructionScript
  (bind _maxintensity (Variables|Default|GetMaxIntensity))
  (bind _sourceheight (Variables|Default|GetSourceHeight))
  (bind _sourceheight_2 (Variables|Default|GetSourceHeight))
  (bind _returnvalue (/ 1e+03 _maxintensity))
  (bind _returnvalue_2 (/ _sourceheight _returnvalue))
  (Class|RectLightComponent|SetSourceHeight (Variables|Default|GetRectLight) _sourceheight_2)
  (Class|RectLightComponent|SetSourceHeight (Variables|Default|GetRectLight1) _sourceheight_2)
  (Rendering|Components|Light|SetIntensity (Variables|Default|GetRectLight) _returnvalue_2)
  (Rendering|Components|Light|SetIntensity (Variables|Default|GetRectLight1) _returnvalue_2))
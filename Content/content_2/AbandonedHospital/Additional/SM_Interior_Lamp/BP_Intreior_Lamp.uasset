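; BP_Intreior_Lamp is an interior lamp Blueprint for the AbandonedHospital content, with adjustable shape and lighting.
; Its construction script applies exposed variables to a spring arm's length, a spot light's cone and attenuation radius, and an additional light's visibility and intensity.
; The event graph holds only disabled placeholder events, so the Blueprint adds no runtime logic.
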(event EventBeginPlay)

(event Collision|EventActorBeginOverlap
  (params (OtherActor :type Actor%20Object%20Reference)))

(event EventTick
  (params (DeltaSeconds :type Float%20%28single-precision%29)))

(fn ConstructionScript
  (Utilities|FlowControl|Sequence
    (:then_0
      (Variables|/Script/Engine.SpringArmComponent|SetTargetArmLength (Variables|Default|GetSpringArm) (Variables|Default|GetTargetArmLength)))
    (:then_1
      (Rendering|SetVisibility (Variables|Default|GetAdditionalLight) (Variables|Default|GetEnableAdditionalLight) false))
    (:then_2
      (Rendering|Components|Light|SetIntensity (Variables|Default|GetAdditionalLight) (Variables|Default|GetIntensityAdditionalLight)))
    (:then_3
      (Rendering|Lighting|SetOuterConeAngle (Variables|Default|GetSpotLight) (Variables|Default|GetConeAngle)))
    (:then_4
      (Rendering|Lighting|SetAttenuationRadius (Variables|Default|GetSpotLight) (Variables|Default|GetAttenuationRadius)))))
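; Interactable data server prop for the Abandoned Hospital content that gives a glitch-and-sparks reaction when used.
; Hover events set and clear an outline overlay material on the server's ward indicator mesh.
; The main action plays a 2D glitch sound and runs the spark particles briefly before deactivating them after a delay.
; Availability queries enable interaction and the main action only, with focus, hold and secondary actions disabled.
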(event EventOnHoverStart
  (params (CurrentControlLayout :type E_ControlLayout%20Enum :default "NewEnumerator0"))
  (bind _sm_dataserver_wardindicator (Variables|Default|GetSM_DataServer_WardIndicator))
  (Rendering|Material|SetOverlayMaterial _sm_dataserver_wardindicator "/Game/content_2/InteractiveObject/Effects/MI_Outline.MI_Outline" :!class /Script/Engine.MeshComponent)
  (Rendering|Material|SetOverlayMaterial _sm_dataserver_wardindicator "/Game/content_2/InteractiveObject/Effects/MI_Outline.MI_Outline" :!class /Script/Engine.MeshComponent))

(event EventOnHoverEnd
  (params (CurrentControlLayout :type E_ControlLayout%20Enum :default "NewEnumerator0"))
  (bind _sm_dataserver_wardindicator (Variables|Default|GetSM_DataServer_WardIndicator))
  (Rendering|Material|SetOverlayMaterial _sm_dataserver_wardindicator 0 :!class /Script/Engine.MeshComponent)
  (Rendering|Material|SetOverlayMaterial _sm_dataserver_wardindicator 0 :!class /Script/Engine.MeshComponent))

(event EventDoMainAction
  (params (HitResult :type Hit%20Result%20Structure))
  (bind _p_sparks_c (Variables|Default|GetP_Sparks_C))
  (Audio|PlaySound2D "/Game/content_2/PlayerAuraEffect/Audio/Sounds_Wav/A_Glitch01.A_Glitch01" 1.0 1.0 0.0 0 0)
  (Components|Activation|Activate _p_sparks_c false)
  (Utilities|FlowControl|Delay 0.8)
  (Components|Activation|Deactivate _p_sparks_c))

(fn ConstructionScript)

(fn IsFocusAvailable
  (return false))

(fn IsInteractionAvailable
  (return true))

(fn IsMainActionAvailable
  (return true))

(fn IsMainHoldActionAvailable
  (return false))

(fn IsSecondActionAvailable
  (return false))

(fn IsSecondHoldActionAvailable
  (return false))
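; Automatic hospital reception door that animates when the player is nearby and shows locked indicators instead if locked.
; Proxy_B overlaps set a ready flag, which a looping timer polls to play the door animations.
; Paired DoOnce gates with delays keep opening and closing from retriggering mid-animation.
; While locked, overlaps fade two WB_Locked widget components in and out rather than moving the door.
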(event OnComponentBeginOverlap(Proxy_B)
  (params (OverlappedComponent :type Primitive%20Component%20Object%20Reference) (OtherActor :type Actor%20Object%20Reference) (OtherComp :type Primitive%20Component%20Object%20Reference) (OtherBodyIndex :type Integer) (bFromSweep :type Boolean) (SweepResult :type Hit%20Result%20Structure%20%28by%20ref%29))
  (Variables|Default|SetReadyToOpen? true)
  (if (Variables|Default|GetLocked?)
    (Default|PlayFadein (Variables|Default|GetWB_Locked_01))
    (Rendering|SetVisibility (Variables|Default|GetLocked_A) true false)))

(event OnComponentEndOverlap(Proxy_B)
  (params (OverlappedComponent :type Primitive%20Component%20Object%20Reference) (OtherActor :type Actor%20Object%20Reference) (OtherComp :type Primitive%20Component%20Object%20Reference) (OtherBodyIndex :type Integer))
  (Variables|Default|SetReadyToOpen? false)
  (if (Variables|Default|GetLocked?)
    (Default|PlayFadeOut (Variables|Default|GetWB_Locked_01))
    (Utilities|FlowControl|Delay 1.0)
    (Rendering|SetVisibility (Variables|Default|GetLocked_A) false false)))

(event Custom|OpenDoor
  (if (not (Variables|Default|GetLocked?))
    (if (Variables|Default|GetReadyToOpen?)
      (Utilities|FlowControl|DoOnce false :!label _label
        (:Completed
          (Components|Animation|PlayAnimation (Variables|Default|GetSM_FloorOne_ReceptionDoor_01) 0 false)
          (Utilities|FlowControl|Delay 1.5)
          (goto _label_2 Reset)))
      (else
        (Utilities|FlowControl|DoOnce true :!label _label_2
          (:Completed
            (Components|Animation|PlayAnimation (Variables|Default|GetSM_FloorOne_ReceptionDoor_01) 0 false)
            (Utilities|FlowControl|Delay 1.5)
            (goto _label Reset)))))))

(event EventBeginPlay
  (Utilities|Casting|CastTo (Game|GetPlayerCharacter 0))
  (Input|EnableInput (Game|GetPlayerController 0))
  (Utilities|Time|SetTimerbyFunctionName 0 "OpenDoor" 0.1 true)
  (bind _aswb_locked (Utilities|Casting|CastToWB_Locked (UserInterface|GetUserWidgetObject (Variables|Default|GetLocked_A))))
  (Variables|Default|SetWB_Locked_01 _aswb_locked)
  (bind _aswb_locked_2 (Utilities|Casting|CastToWB_Locked (UserInterface|GetUserWidgetObject (Variables|Default|GetLocked_B))))
  (Variables|Default|SetWB_Locked_02 _aswb_locked_2))

(event Collision|EventActorBeginOverlap
  (params (OtherActor :type Actor%20Object%20Reference)))

(event EventTick
  (params (DeltaSeconds :type Float%20%28single-precision%29)))

(fn ConstructionScript)
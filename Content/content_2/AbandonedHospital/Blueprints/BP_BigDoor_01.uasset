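; BP_BigDoor_01 is an AbandonedHospital double door that shows "Press E" or "Locked" prompts when something overlaps its proximity component.
; Paired widgets fade in on overlap and fade out before hiding, chosen by the Locked flag.
; Open/close animation logic checks Locked and ReadyToOpen, using FlipFlop, DoOnce gates and delays.
; That logic and the input/widget-reference setup have no triggering event here, so neither runs.
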(event OnComponentBeginOverlap(Proxy_B)
  (params (OverlappedComponent :type Primitive%20Component%20Object%20Reference) (OtherActor :type Actor%20Object%20Reference) (OtherComp :type Primitive%20Component%20Object%20Reference) (OtherBodyIndex :type Integer) (bFromSweep :type Boolean) (SweepResult :type Hit%20Result%20Structure%20%28by%20ref%29))
  (Variables|Default|SetReadyToOpen? true)
  (if (Variables|Default|GetLocked?)
    (Default|PlayFadein (Variables|Default|GetWB_Locked_01))
    (Rendering|SetVisibility (Variables|Default|GetLocked_A) true false)
    (else
      (Default|PlayFadein (Variables|Default|GetWB_PressE_01))
      (Rendering|SetVisibility (Variables|Default|GetPressE_A) true false))))

(event OnComponentEndOverlap(Proxy_B)
  (params (OverlappedComponent :type Primitive%20Component%20Object%20Reference) (OtherActor :type Actor%20Object%20Reference) (OtherComp :type Primitive%20Component%20Object%20Reference) (OtherBodyIndex :type Integer))
  (Variables|Default|SetReadyToOpen? false)
  (if (Variables|Default|GetLocked?)
    (Default|PlayFadeOut (Variables|Default|GetWB_Locked_01))
    (Utilities|FlowControl|Delay 1.0)
    (Rendering|SetVisibility (Variables|Default|GetLocked_A) false false)
    (else
      (Default|PlayFadeOut (Variables|Default|GetWB_PressE_01))
      (Utilities|FlowControl|Delay 1.0)
      (Rendering|SetVisibility (Variables|Default|GetPressE_A) false false))))

(event EventBeginPlay)

(event Collision|EventActorBeginOverlap
  (params (OtherActor :type Actor%20Object%20Reference)))

(event EventTick
  (params (DeltaSeconds :type Float%20%28single-precision%29)))

(fn ConstructionScript)
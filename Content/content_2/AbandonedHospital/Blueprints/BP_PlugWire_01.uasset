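; Plug wire prop for the abandoned hospital set that lays a wire along an editable spline, with no active gameplay logic.
; The construction script divides the spline into sections sized by the actor's Z scale and adds a Z-forward spline mesh for each, with a fixed offset and rotation.
; Each segment takes its endpoints and tangents from the spline, with tangents clamped to section length.
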(event EventBeginPlay)

(event Collision|EventActorBeginOverlap
  (params (OtherActor :type Actor%20Object%20Reference)))

(event EventTick
  (params (DeltaSeconds :type Float%20%28single-precision%29)))

(fn ConstructionScript
  (bind _spline (Variables|Default|GetSpline))
  (bind _spline_2 (Variables|Default|GetSpline))
  (Variables|Default|SetSection_length (* (.z (Transformation|GetActorScale3D)) 1e+01))
  (for _index (range 0 (Math|Float|Truncate (/ (Spline|GetSplineLength (Variables|Default|GetSpline)) (Variables|Default|GetSection_length))))
    (bind _returnvalue (AddComponent|AddSplineMeshComponent false))
    (Transformation|AddRelativeLocation _returnvalue "2.652595,0.000000,-4.189266" false false)
    (Transformation|AddLocalRotation _returnvalue "-90.000000,0.000000,0.000000" false false)
    (SplineMesh|SetForwardAxis _returnvalue "Z" true)
    (SplineMesh|SetStartandEnd _returnvalue (Spline|GetLocationatDistanceAlongSpline _spline (* _index (Variables|Default|GetSection_length)) "Local") (Math|Vector|ClampVectorSize (Spline|GetTangentatDistanceAlongSpline _spline (* _index (Variables|Default|GetSection_length)) "Local") 0.0 (Variables|Default|GetSection_length)) (Spline|GetLocationatDistanceAlongSpline _spline_2 (* (+ _index 1) (Variables|Default|GetSection_length)) "Local") (Math|Vector|ClampVectorSize (Spline|GetTangentatDistanceAlongSpline _spline_2 (* (+ _index 1) (Variables|Default|GetSection_length)) "Local") 0.0 (Variables|Default|GetSection_length)) true :!class /Script/Engine.SplineMeshComponent)))